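; Enemy character that roams by a default AI movement mode and switches to chasing a pawn it spots through PawnSensing, if chasing is enabled.
; Tick drops the target and restores default movement once it exceeds the lose-sight distance.
; Getters expose movement type, chase target, patrol, wander and decision-wait settings.
; Initiating contact destroys the enemy and its controller, then asks MyGameState to start a test battle.
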(event `self.ReceiveBeginPlay`
  (set `self.Current AI Movement` (`self.Default AI Movement`)))

(event `self.ReceiveTick`
  (params (DeltaSeconds :type "Float (single-precision)"))
  (bind _chase_target (`self.Chase Target`))
  (if (!= _chase_target null)
    (if (> (`self.GetDistanceTo` _chase_target) (`self.Lose Sight Distance`))
      (set `self.Chase Target` null)
      (set `self.Current AI Movement` (`self.Default AI Movement`))
      (`KismetSystemLibrary.PrintString` "lost sight"))))

(event `self.PawnSensing.OnSeePawn`
  (params (Pawn :type "Pawn Object Reference"))
  (if (`self.Chases`)
    (set `self.Chase Target` Pawn)
    (set `self.Current AI Movement` "NewEnumerator4")
    (`KismetSystemLibrary.PrintString` "target found")))

(fn `Get Chase Target`
  (returns (Chasing :type Boolean) (`Chase Target` :type "Actor Object Reference"))
  (bind _chase_target (`self.Chase Target`))
  (return (!= _chase_target null) _chase_target))

(fn `Get Decision Wait Time`
  (returns (Time :type "Float (double-precision)"))
  (return (`KismetMathLibrary.RandomFloatInRange` (`self.Decision Time Min`) (`self.Decision Time Max`))))

(fn `Get Desired AI Type`
  (returns (Type :type "/Game/Blueprints/Data/AIMovementType Enum"))
  (return (`self.Current AI Movement`)))

(fn `Get Patrol Points`
  (returns (`Patrol Points` :type "Array of /Game/Blueprints/WayPoint Object Reference"))
  (return (`self.Patrol Points`)))

(fn `Get True Wander`
  (returns (`True Wander` :type Boolean))
  (return (`self.True Wander`)))

(fn `Get Wander Range`
  (returns (Range :type Integer))
  (return (`self.Wander Range`)))

(fn `Initiate Contact`
  (params (Actor :type "Actor Object Reference"))
  (returns (Success :type Boolean))
  (`self.K2_DestroyActor` (`self.GetController`))
  (`self.K2_DestroyActor`)
  (bind _asmy_game_state (cast `/Game/MyGameState` (`GameplayStatics.GetGameState`))
    (:`then`
      (`/Game/MyGameState.Initiate Test Battle` _asmy_game_state)
      (return true))
    (:`CastFailed`
      (return false))))

(fn `UserConstructionScript`)