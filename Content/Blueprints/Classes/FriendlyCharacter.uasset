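; FriendlyCharacter is an NPC character that billboards to the camera and can chase pawns it sees.
; PawnSensing sets the chase target and switches the movement mode, which Tick restores to default beyond a lose-sight distance.
; Getter functions expose movement, patrol, wander and decision-timing settings.
; ExplorerCharacter overlap swaps the sphere for a material billboard, while dialog, choice and interaction functions are mostly stubs, with BeginEvent calling MyHUD.
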(event `self.ReceiveBeginPlay`
  (set `self.Current AI Movement` (`self.Default AI Movement`)))

(event `self.ReceiveTick`
  (params (DeltaSeconds :type "Float (single-precision)"))
  (bind _chase_target (`self.Chase Target`))
  (`self.Update Billboarding`)
  (if (!= _chase_target null)
    (if (> (`self.GetDistanceTo` _chase_target) (`self.Lose Sight Distance`))
      (set `self.Chase Target` null)
      (set `self.Current AI Movement` (`self.Default AI Movement`))
      (`KismetSystemLibrary.PrintString` "lost sight"))))

(event `self.PawnSensing.OnSeePawn`
  (params (Pawn :type "Pawn Object Reference"))
  (if (`self.Chases`)
    (set `self.Chase Target` Pawn)
    (set `self.Current AI Movement` "NewEnumerator4")
    (`KismetSystemLibrary.PrintString` "target found")))

(event `self.ReceiveActorBeginOverlap`
  (params (OtherActor :type "Actor Object Reference"))
  (cast `/Game/Blueprints/Classes/ExplorerCharacter` OtherActor)
  (`SceneComponent.SetVisibility` (`self.MaterialBillboard`) true false)
  (`SceneComponent.SetVisibility` (`self.Sphere`) false false))

(event `self.ReceiveActorEndOverlap`
  (params (OtherActor :type "Actor Object Reference"))
  (cast `/Game/Blueprints/Classes/ExplorerCharacter` OtherActor)
  (`SceneComponent.SetVisibility` (`self.MaterialBillboard`) false false)
  (`SceneComponent.SetVisibility` (`self.Sphere`) true false))

(fn `ActivateInteraction`
  (params (Activator :type "Actor Object Reference"))
  (returns (Success :type Boolean))
  (return false))

(fn `Begin Event`
  (bind _asmy_hud (cast `/Game/MyHUD` (`PlayerController.GetHUD` (`GameplayStatics.GetPlayerController` 0))))
  (`/Game/MyHUD.Wants World Event` _asmy_hud self)
  (return))

(fn `Choice Made`
  (params (Index :type Integer))
  (returns (Success :type Boolean))
  (return false))

(fn `Conclude Event`
  (returns (`Is Finished` :type Boolean))
  (return true))

(fn `Get Chase Target`
  (returns (Chasing :type Boolean) (`Chase Target` :type "Actor Object Reference"))
  (bind _chase_target (`self.Chase Target`))
  (return (!= _chase_target null) _chase_target))

(fn `Get Choices`
  (returns (Choices :type "Array of String") (`Cancel Index` :type Integer))
  (return _ -1))

(fn `Get Decision Wait Time`
  (returns (Time :type "Float (double-precision)"))
  (return (`KismetMathLibrary.RandomFloatInRange` (`self.Decision Time Min`) (`self.Decision Time Max`))))

(fn `Get Desired AI Type`
  (returns (Type :type "/Game/Blueprints/Data/AIMovementType Enum"))
  (return (`self.Current AI Movement`)))

(fn `Get Dialog`
  (returns (Success :type Boolean) (Dialog :type "/Game/Blueprints/Data/Dialog Structure"))
  (return false))

(fn `Get Patrol Points`
  (returns (`Patrol Points` :type "Array of /Game/Blueprints/WayPoint Object Reference"))
  (return (`self.Patrol Points`)))

(fn `Get True Wander`
  (returns (`True Wander` :type Boolean))
  (return (`self.True Wander`)))

(fn `Get Wander Range`
  (returns (Range :type Integer))
  (return (`self.Wander Range`)))

(fn `Initiate Contact`
  (params (Actor :type "Actor Object Reference"))
  (returns (Success :type Boolean))
  (return true))

(fn `Update Billboarding`
  (`self.K2_SetActorRotation` (`PlayerCameraManager.GetCameraRotation` (`PlayerController.PlayerCameraManager` (`GameplayStatics.GetPlayerController` 0)))))

(fn `UserConstructionScript`)

(fn `Wants Choices`
  (returns (`Wants Choices` :type Boolean))
  (bind _choices (`self.Get Choices`))
  (return (> (`KismetArrayLibrary.Array_Length` _choices) 0)))