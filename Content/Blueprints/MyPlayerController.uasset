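; Player controller for grid-based, first-person-style exploration with tile steps and 90-degree turns.
; Axis input passes gate macros for idle, UI and play state; moves also require an unoccupied TileManager tile.
; Tick lerps location or control rotation to the target, applying poison damage and eventual recovery after each completed step.
; Confirm or left click line-traces for Interactables, Menu toggles operations, and temporary debug keys trigger a test battle or grant materials.
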(event `self.ReceiveBeginPlay`
  (bind _returnvalue (`self.K2_GetPawn`))
  (set `self.Previous Rotation` (`self.GetControlRotation`))
  (`/Engine/EditorBlueprintResources/StandardMacros.IsValid` _returnvalue
    (:`Is Valid`
      (`KismetSystemLibrary.Delay` 0.5)
      (set `self.Previous Location` (`self.K2_GetActorLocation` _returnvalue)))))

(event `self.ReceiveTick`
  (params (DeltaSeconds :type "Float (single-precision)"))
  (switch `/Game/Blueprints/Data/MovementState` (`self.Movement State`)
    (:`NewEnumerator1`
      (bind _did_finish (`self.Update Movement`))
      (if _did_finish
        (`self.Update Status Effects`)))
    (:`NewEnumerator2`
      (`self.Update Turning`))))

(event `Key|Seven`
  (params (Key :type "Key Structure"))
  ;[1 1 1] TODO KILL ME!
  (:`Pressed`
    (bind _asmy_game_state (cast `/Game/MyGameState` (`GameplayStatics.GetGameState`)))
    (`/Game/MyGameState.Initiate Test Battle` _asmy_game_state)))

(event `InputAxis|Turn` :consume false
  (params (AxisValue :type "Float (single-precision)"))
  ;[1 1 1] Turn
  (`self.Turn Enabled` AxisValue
    (:`true`
      (set `self.Desired Rotation` (`KismetMathLibrary.ComposeRotators` (`self.Previous Rotation`) (`KismetMathLibrary.MakeRotator` 0.0 0.0 (* 90.0 AxisValue))))
      (set `self.Movement State` "NewEnumerator2")
      (set `self.Step` 0.0))))

(event `InputAxis|Strafe` :consume false
  (params (AxisValue :type "Float (single-precision)"))
  ;[1 1 1] Strafe
  (`self.Do Input Axis` (`KismetMathLibrary.GetRightVector` (`self.Previous Rotation`)) AxisValue))

(event `InputAxis|Move` :consume false
  (params (AxisValue :type "Float (single-precision)"))
  ;[1 1 1] Move
  (`self.Do Input Axis` (`KismetMathLibrary.GetForwardVector` (`self.Previous Rotation`)) AxisValue))

(event `Key|Eight`
  (params (Key :type "Key Structure"))
  ;[1 1 1] DELETE MEFree Items
  (:`Pressed`
    (bind _asmy_game_state (cast `/Game/MyGameState` (`GameplayStatics.GetGameState`)))
    (`/Game/MyGameState.Aquired Inventory` _asmy_game_state (`|MakeArray`) (`|MakeArray` (make `/Game/Blueprints/Data/WorldMaterial` "Blub Blub" "Fux" 1) (make `/Game/Blueprints/Data/WorldMaterial` "Ooze" "From the land of ooooOO!" 1)))))

(event `InputAction|Menu`
  (params (Key :type "Key Structure"))
  ;[1 1 1] Operations Menu
  (:`Pressed`
    (`self.Interface Not Busy`
      (:`true`
        (bind _asmy_game_state (cast `/Game/MyGameState` (`GameplayStatics.GetGameState`)))
        (`/Game/MyGameState.Toggle Operations Menu` _asmy_game_state)))))

(event `InputAction|Confirm` :consume false
  (params (Key :type "Key Structure"))
  (bind _rootcomponent (`Actor.RootComponent` (`self.K2_GetPawn`)))
  (bind _returnvalue (`SceneComponent.K2_GetComponentLocation` _rootcomponent))
  ;[1 1 1] Activate Interactables
  (:`Pressed`
    (`self.Is Exploring` :!label _label
      (:`true`
        (`self.Interface Not Busy`
          (:`true`
            (bind _outhit (`KismetSystemLibrary.LineTraceSingle` :`Start` _returnvalue :`End` (+ _returnvalue (* (`KismetMathLibrary.GetForwardVector` (`SceneComponent.K2_GetComponentRotation` _rootcomponent)) 400.0)) :`TraceChannel` "TraceTypeQuery1" :`DrawDebugType` "ForDuration"))
            (bind (_bblockinghit _binitialoverlap _time _location _impactpoint _normal _impactnormal _physmat _hitactor) (`GameplayStatics.BreakHitResult` _outhit))
            (`KismetSystemLibrary.PrintString` (`KismetSystemLibrary.GetDisplayName` _hitactor))
            (bind _asinteractable (cast `/Game/Blueprints/Interfaces/Interactable` _hitactor))
            (`/Game/Blueprints/Interfaces/Interactable.ActivateInteraction` _asinteractable self)))))))

(event `Key|LeftMouseButton`
  (params (Key :type "Key Structure"))
  ;[1 1 1] Activate Interactables
  (:`Pressed`
    (goto _label)))

(fn `Do Input Axis`
  (params (A :type "Vector Structure") (A2 :type "Float (double-precision)"))
  (bind _previous_location (`self.Previous Location`))
  (bind _returnvalue (+ _previous_location (* A (* A2 400.0))))
  (`self.Input is 1` A2
    (:`true`
      (`self.Interface Not Busy`
        (:`true`
          (`self.Is Exploring`
            (:`true`
              (bind _manager (`/Game/Blueprints/Utility/HelperLib.Get Tile Manager`))
              (bind (_found _tile) (`/Game/Blueprints/TileManager.Get Tile at Vector` _manager _returnvalue))
              (if _found
                (bind _occupied (`/Game/Blueprints/Tile.Is Occupied` _tile))
                (if (not _occupied)
                  (set `self.Movement State` "NewEnumerator1")
                  (set `self.Step` 0.0)
                  (set `self.Previous Location` _previous_location)
                  (set `self.Desired Location` _returnvalue))))))))))

(fn `Update Movement`
  (returns (`Did Finish` :type Boolean))
  (bind _returnvalue (`self.K2_GetPawn`))
  (bind _ascharacter (cast `Character` _returnvalue))
  (bind _output_get (set `self.Step` (`KismetMathLibrary.FClamp` (+ (`self.Step`) (* (`MovementComponent.GetMaxSpeed` (`Character.CharacterMovement` _ascharacter)) (`GameplayStatics.GetWorldDeltaSeconds`))) 0.0 400.0)))
  (bind _returnvalue_2 (/ _output_get 400.0))
  (`self.K2_SetActorLocation` _returnvalue (`KismetMathLibrary.VLerp` (`self.Previous Location`) (`self.Desired Location`) _returnvalue_2) false false)
  (bind _returnvalue_3 (>= _returnvalue_2 1.0))
  (if _returnvalue_3
    (set `self.Previous Location` (`self.Desired Location`))
    (set `self.Movement State` "NewEnumerator0"))
  (return _returnvalue_3))

(fn `Update Status Effects`
  (bind _asmy_game_state (cast `/Game/MyGameState` (`GameplayStatics.GetGameState`)))
  (bind _player (`/Game/MyGameState.Player` _asmy_game_state))
  (switch `/Game/Blueprints/Data/BattleFighterStatus` (`.Status_83_FA2CFAFB48AC061028B449B41B9440AC` (break `/Game/Blueprints/Data/BattleFighter` _player))
    (:`NewEnumerator1`
      (bind (_name _owningtarget _status _strength _intellect _agility _healthmax _healthcurrent) (break `/Game/Blueprints/Data/BattleFighter` _player))
      (setmembers `/Game/Blueprints/Data/BattleFighter` :`StructRef` _player :`Health Current` (- _healthcurrent (`KismetMathLibrary.FTrunc` (* _healthmax 0.02))))
      (`GameplayStatics.PlayWorldCameraShake` "/Game/Blueprints/DamagedShake.DamagedShake_C" (`self.K2_GetActorLocation` (`GameplayStatics.GetPlayerCharacter` 0)) 0.0 400.0)
      (bind _result (`/Engine/EditorBlueprintResources/StandardMacros.IncrementInt` (`self.Poison Step Counter`))
        (:`  `
          (if (>= _result 10)
            (setmembers `/Game/Blueprints/Data/BattleFighter` :`StructRef` _player :`Status` "NewEnumerator6")
            (`/Game/MyGameState.Wants Results Dialog` _asmy_game_state (`|MakeArray` (make `/Game/Blueprints/Data/BattleResult` "NewEnumerator0" "{owner} recovered from Poison.")))))))))

(fn `Update Turning`
  (returns (`Did Finish` :type Boolean))
  (bind _output_get (set `self.Step` (`KismetMathLibrary.FClamp` (+ (`self.Step`) (* (`self.Turn Rate`) (`GameplayStatics.GetWorldDeltaSeconds`))) 0.0 90.0)))
  (bind _returnvalue (/ _output_get 90.0))
  (`self.SetControlRotation` (`KismetMathLibrary.RLerp` (`self.Previous Rotation`) (`self.Desired Rotation`) _returnvalue true))
  (bind _returnvalue_2 (>= _returnvalue 1.0))
  (if _returnvalue_2
    (set `self.Previous Rotation` (`self.Desired Rotation`))
    (set `self.Movement State` "NewEnumerator0"))
  (return _returnvalue_2))

(fn `UserConstructionScript`)