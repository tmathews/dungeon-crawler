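; AI controller that moves a ControllableCharacter tile by tile, patrolling, wandering or chasing according to its desired AI type.
; Paths come from the TileManager, with wander goals picked randomly by box trace and chase paths rebuilt every step.
; Tick runs a None/Turning/Moving state machine while PlayState is 0, lerping rotation and location manually.
; An occupied next tile triggers contact with its occupant; failed pathing waits via a dispatcher before retrying.
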(event `self.ReceiveBeginPlay`
  (`KismetSystemLibrary.Delay` 2.0)
  (bind _output_get (set `self.Start Location` (`self.K2_GetActorLocation` (`self.K2_GetPawn`))))
  (set `self.Previous Location` _output_get)
  (set `self.Current Rotation` (`self.GetControlRotation`))
  (add `self.Wait for Decision` (delegate `On Wait For Decision`))
  (set `self.Is Waiting` false))

(event `On Wait For Decision` :!signature `self.Wait for Decision`
  (params (Delay :type "Float (double-precision)"))
  (set `self.Is Waiting` true)
  (`KismetSystemLibrary.Delay` Delay)
  (set `self.Is Waiting` false)
  (`self.Initiate Movement`))

(event `self.ReceiveTick`
  (params (DeltaSeconds :type "Float (single-precision)"))
  (bind _asmy_game_state (cast `/Game/MyGameState` (`GameplayStatics.GetGameState`)))
  (if (and (== (`/Game/MyGameState.Play State` _asmy_game_state) 0) (not (`self.Is Waiting`)))
    (switch `/Game/Blueprints/Data/MovementState` (`self.Movement State`)
      (:`NewEnumerator0`
        (bind _done (`self.Is Done Path`))
        (if _done
          (`self.Initiate Movement` :!label _label)
          (else
            (bind _ascontrollable_character (cast `/Game/Blueprints/Interfaces/ControllableCharacter` (`self.K2_GetPawn`)))
            (bind _type (`/Game/Blueprints/Interfaces/ControllableCharacter.Get Desired AI Type` _ascontrollable_character))
            (if (`|EnumEquality` _type "NewEnumerator4")
              (goto _label)
              (else
                (`self.Start Movement`))))))
      (:`NewEnumerator1`
        (`self.Update Movement`))
      (:`NewEnumerator2`
        (`self.Update Turning`)))))

(fn `Collides with Tile`
  (params (`Tile Position` :type "Vector Structure"))
  (returns (Collides :type Boolean))
  (bind _outhits (`KismetSystemLibrary.LineTraceMultiForObjects` :`Start` (`self.K2_GetActorLocation` (`self.K2_GetPawn`)) :`End` `Tile Position` :`ObjectTypes` (`|MakeArray` "ObjectTypeQuery1" :!type "EObjectTypeQuery Enum") :`DrawDebugType` "ForDuration"))
  (for _array_element _outhits
    (bind (_bblockinghit _binitialoverlap _time _location _impactpoint _normal _impactnormal _physmat _hitactor) (`GameplayStatics.BreakHitResult` _array_element))
    (cast `/Game/Blueprints/Tile` _hitactor)
    (if _bblockinghit
      (return true)))
  (return false))

(fn `Get New Chase Path`
  (returns (Found :type Boolean))
  (bind _ascontrollable_character (cast `/Game/Blueprints/Interfaces/ControllableCharacter` (`self.K2_GetPawn`)))
  (bind (_chasing _chase_target) (`/Game/Blueprints/Interfaces/ControllableCharacter.Get Chase Target` _ascontrollable_character))
  (if _chasing
    (bind _found (`self.Set New Current Path` _chase_target))
    (return _found)
    (else
      (return false))))

(fn `Get New Patrol Path`
  (returns (Success :type Boolean))
  (bind _ascontrollable_character (cast `/Game/Blueprints/Interfaces/ControllableCharacter` (`self.K2_GetPawn`)))
  (bind _patrol_points (`/Game/Blueprints/Interfaces/ControllableCharacter.Get Patrol Points` _ascontrollable_character))
  (bind _output_get (set `self.Patrol Points` _patrol_points))
  (bind _found (`self.Set New Current Path` (`|GetArrayItem` _output_get (`self.Patrol Index`))))
  (set `self.Patrol Index` (mod (+ (`self.Patrol Index`) 1) (`KismetArrayLibrary.Array_Length` (`self.Patrol Points`))))
  (return _found))

(fn `Get New Wander Path`
  (returns (Success :type Boolean))
  (locals (tArr :type "Array of Actor Object Reference"))
  (bind _returnvalue (`self.K2_GetPawn`))
  (bind _tarr (`local.tArr`))
  (if (`KismetMathLibrary.RandomBool`)
    (bind _ascontrollable_character (cast `/Game/Blueprints/Interfaces/ControllableCharacter` _returnvalue))
    (bind _true_wander (`/Game/Blueprints/Interfaces/ControllableCharacter.Get True Wander` _ascontrollable_character))
    (bind _range (`/Game/Blueprints/Interfaces/ControllableCharacter.Get Wander Range` _ascontrollable_character))
    (bind _returnvalue_2 (select `bool` _true_wander :`false` (`self.Start Location`) :`true` (`self.K2_GetActorLocation` _returnvalue)))
    (bind _returnvalue_3 (`KismetMathLibrary.Conv_IntToDouble` _range))
    (bind _outhits (`KismetSystemLibrary.BoxTraceMulti` :`Start` _returnvalue_2 :`End` _returnvalue_2 :`HalfSize` (`KismetMathLibrary.MakeVector` _returnvalue_3 _returnvalue_3 100.0) :`TraceChannel` "TraceTypeQuery1" :`DrawDebugType` "ForDuration"))
    (for _array_element _outhits
      (bind _astile (cast `/Game/Blueprints/Tile` (`.HitActor` (`GameplayStatics.BreakHitResult` _array_element))))
      (`KismetArrayLibrary.Array_Add` (`local.tArr`) _astile))
    (bind _found (`self.Set New Current Path` (`|GetArrayItem` _tarr (`KismetMathLibrary.RandomInteger` (`KismetArrayLibrary.Array_Length` _tarr)))))
    (return _found)
    (else
      (return false))))

(fn `Initiate Movement`
  (bind _ascontrollable_character (cast `/Game/Blueprints/Interfaces/ControllableCharacter` (`self.K2_GetPawn`)))
  (bind _type (`/Game/Blueprints/Interfaces/ControllableCharacter.Get Desired AI Type` _ascontrollable_character))
  (switch `/Game/Blueprints/Data/AIMovementType` _type
    (:`NewEnumerator2`
      (bind _success (`self.Get New Patrol Path`))
      (if _success
        (`self.Start Movement` :!label _label)
        (else
          (bind _time (`/Game/Blueprints/Interfaces/ControllableCharacter.Get Decision Wait Time` _ascontrollable_character :!label _label_2))
          (`self.Wait for Decision` _time))))
    (:`NewEnumerator3`
      (bind _success_2 (`self.Get New Wander Path`))
      (if _success_2
        (goto _label)
        (else
          (goto _label_2))))
    (:`NewEnumerator4`
      (bind _found (`self.Get New Chase Path`))
      (if _found
        (goto _label)
        (else
          (`self.Wait for Decision` 1.0))))))

(fn `Is Done Path`
  (returns (Done :type Boolean))
  (return (and (== (`KismetArrayLibrary.Array_Length` (`self.Current Path`)) 0) (`|EnumEquality` (`self.Movement State`) "NewEnumerator0"))))

(fn `Set New Current Path`
  (params (Goal :type "Actor Object Reference"))
  (returns (Found :type Boolean))
  (locals (tArr :type "Array of Vector Structure"))
  (bind _manager (`/Game/Blueprints/Utility/HelperLib.Get Tile Manager`))
  (`KismetArrayLibrary.Array_Clear` (`self.Current Path`))
  (bind _path (`/Game/Blueprints/TileManager.Vector Path to Actor` _manager (`self.K2_GetPawn`) Goal))
  (bind _output_get (set `local.tArr` _path))
  (`KismetArrayLibrary.Array_Remove` _output_get (- (`KismetArrayLibrary.Array_Length` _output_get) 1))
  (bind (_arrayindex _arrayelement) (`/Engine/EditorBlueprintResources/StandardMacros.ReverseForEachLoop` _output_get)
    (:`LoopBody`
      (`KismetArrayLibrary.Array_Add` (`self.Current Path`) (`KismetMathLibrary.MakeVector` (.x _arrayelement) (.y _arrayelement) (.z (`self.Start Location`)))))
    (:`Completed`
      (return (> (`KismetArrayLibrary.Array_Length` (`self.Current Path`)) 0)))))

(fn `Start Movement`
  (bind _current_path (`self.Current Path`))
  (bind _output (`|GetArrayItem` _current_path))
  (bind _returnvalue (`KismetMathLibrary.FindLookAtRotation` (`self.Previous Location`) _output))
  (if (> (`KismetArrayLibrary.Array_Length` _current_path) 0)
    (bind _manager (`/Game/Blueprints/Utility/HelperLib.Get Tile Manager`))
    (bind (_found _tile) (`/Game/Blueprints/TileManager.Get Tile at Vector` _manager _output))
    (if _found
      (bind (_occupied _characters) (`/Game/Blueprints/Tile.Is Occupied` _tile))
      (if _occupied
        (bind _ascontrollable_character (cast `/Game/Blueprints/Interfaces/ControllableCharacter` (`self.K2_GetPawn`)))
        (`/Game/Blueprints/Interfaces/ControllableCharacter.Initiate Contact` _ascontrollable_character (`|GetArrayItem` _characters))
        (elif (== (`self.Current Rotation`) _returnvalue)
          (set `self.Desired Location` _output)
          (`KismetArrayLibrary.Array_Remove` _current_path)
          (set `self.Step` 0.0)
          (set `self.Movement State` "NewEnumerator1")
          (else
            (set `self.Desired Rotation` _returnvalue)
            (set `self.Step` 0.0)
            (set `self.Movement State` "NewEnumerator2")))))))

(fn `Update Movement`
  (returns (`Did Finish` :type Boolean))
  (bind _returnvalue (`self.K2_GetPawn`))
  (bind _ascharacter (cast `Character` _returnvalue))
  (bind _output_get (set `self.Step` (`KismetMathLibrary.FClamp` (+ (`self.Step`) (* (`MovementComponent.GetMaxSpeed` (`Character.CharacterMovement` _ascharacter)) (`GameplayStatics.GetWorldDeltaSeconds`))) 0.0 400.0)))
  (bind _returnvalue_2 (/ _output_get 400.0))
  (`self.K2_SetActorLocation` _returnvalue (`KismetMathLibrary.VLerp` (`self.Previous Location`) (`self.Desired Location`) _returnvalue_2) false false)
  (bind _returnvalue_3 (>= _returnvalue_2 1.0))
  (if _returnvalue_3
    (set `self.Previous Location` (`self.Desired Location`))
    (set `self.Movement State` "NewEnumerator0"))
  (return _returnvalue_3))

(fn `Update Turning`
  (returns (`Did Finish` :type Boolean))
  (bind _output_get (set `self.Step` (`KismetMathLibrary.FClamp` (+ (`self.Step`) (* (`self.Turn Rate`) (`GameplayStatics.GetWorldDeltaSeconds`))) 0.0 90.0)))
  (bind _returnvalue (/ _output_get 90.0))
  (`self.SetControlRotation` (`KismetMathLibrary.RLerp` (`self.Current Rotation`) (`self.Desired Rotation`) _returnvalue true))
  (bind _returnvalue_2 (>= _returnvalue 1.0))
  (if _returnvalue_2
    (set `self.Current Rotation` (`self.Desired Rotation`))
    (set `self.Movement State` "NewEnumerator0"))
  (return _returnvalue_2))

(fn `UserConstructionScript`)