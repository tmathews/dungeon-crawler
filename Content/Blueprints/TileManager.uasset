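; Tile manager that turns the placed Tile actors into a flat occupancy grid for pathfinding between actors.
; On BeginPlay it caches the grid, which FindPath uses to return paths as indices or world positions.
; Helpers convert between world locations and grid cells, set up all tiles, and find a Tile by sphere trace.
; PlotGrid rebuilds the cache and spawns TileIndicators visualising empty, tiled and path cells.
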(event `self.ReceiveBeginPlay`
  (bind _grid (`self.Get Grid from Tiles`))
  (set `self.Grid Cache` _grid))

(fn `Actor to Grid Index`
  (params (Actor :type "Actor Object Reference"))
  (returns (Index :type Integer))
  (bind _point (`self.Vector to Grid Point` (`self.K2_GetActorLocation` Actor)))
  (bind _index (`/Game/Blueprints/Utility/PathFindingLib.Point to Index` (`self.Width`) _point))
  (return _index))

(fn `Get Grid from Tiles`
  (returns (Grid :type "Array of Boolean"))
  (locals (tGrid :type "Array of Boolean"))
  (`KismetArrayLibrary.Array_Resize` (`local.tGrid`) (* (`self.Width`) (`self.Height`)))
  (bind _outactors (`GameplayStatics.GetAllActorsOfClass` "/Game/Blueprints/Tile.Tile_C"))
  (for _array_element _outactors
    (bind _index (`self.Actor to Grid Index` _array_element))
    (`KismetArrayLibrary.Array_Set` (`local.tGrid`) _index true))
  (return (`local.tGrid`)))

(fn `Get Tile at Vector`
  (params (Vec3 :type "Vector Structure"))
  (returns (Found :type Boolean) (Tile :type "/Game/Blueprints/Tile Object Reference"))
  (bind _outhits (`KismetSystemLibrary.SphereTraceMulti` Vec3 Vec3 (`KismetMathLibrary.Conv_IntToDouble` (/ (`self.Tile Size`) 4)) "TraceTypeQuery1"))
  (for _array_element _outhits
    (bind _astile (cast `/Game/Blueprints/Tile` (`.HitActor` (`GameplayStatics.BreakHitResult` _array_element))))
    (return true _astile))
  (return false null))

(fn `Grid Point to Vector`
  (params (Point :type "Vector2D Structure"))
  (returns (Vector :type "Vector Structure"))
  (bind (_x _y) (`KismetMathLibrary.BreakVector2D` Point))
  (bind _returnvalue (`KismetMathLibrary.Conv_IntToDouble` (`self.Tile Size`)))
  (bind _returnvalue_2 (`KismetMathLibrary.Conv_IntToDouble` (`self.Offset`)))
  (return (`KismetMathLibrary.MakeVector` (+ (* _x _returnvalue) _returnvalue_2) (+ (* _y _returnvalue) _returnvalue_2))))

(fn `Path to Actor`
  (params (Start :type "Actor Object Reference") (Goal :type "Actor Object Reference"))
  (returns (Path :type "Array of Integer"))
  (bind _index (`self.Actor to Grid Index` Start))
  (bind _index_2 (`self.Actor to Grid Index` Goal))
  (bind _path (`/Game/Blueprints/Utility/PathFindingLib.Find Path` (`self.Grid Cache`) (`self.Width`) _index _index_2))
  (return _path))

(fn `Plot Grid`
  (bind _offset (`self.Offset`))
  (bind _tile_size (`self.Tile Size`))
  (`self.Remove Grid`)
  (bind _grid (`self.Get Grid from Tiles`))
  (bind _output_get (set `self.Grid Cache` _grid))
  (bind _path (`self.Path to Actor` (`self.Start`) (`self.Goal`)))
  (for (_array_element _array_index) _output_get
    (bind _point (`/Game/Blueprints/Utility/PathFindingLib.Index to Point` _array_index (`self.Width`)))
    (bind (_x _y) (`KismetMathLibrary.BreakVector2D` _point))
    (bind _returnvalue (`|SpawnActorFromClass` "/Game/Blueprints/TileIndicator.TileIndicator_C" (`KismetMathLibrary.MakeTransform` (`KismetMathLibrary.MakeVector` (`KismetMathLibrary.Conv_IntToDouble` (+ _offset (* (`KismetMathLibrary.FFloor` _x) _tile_size))) (`KismetMathLibrary.Conv_IntToDouble` (+ _offset (* (`KismetMathLibrary.FFloor` _y) _tile_size))) 200.0)) "Undefined" "OverrideRootScale" null null))
    (`/Game/Blueprints/TileIndicator.Set On` _returnvalue (select `bool` (`KismetArrayLibrary.Array_Contains` _path _array_index) :`false` (select `bool` _array_element :`true` 1 :!type "Byte") :`true` 2))))

(fn `Remove Grid`
  (bind _outactors (`GameplayStatics.GetAllActorsOfClass` "/Game/Blueprints/TileIndicator.TileIndicator_C"))
  (for _array_element _outactors
    (`self.K2_DestroyActor` _array_element)))

(fn `Setup All Tiles`
  (bind _outactors (`GameplayStatics.GetAllActorsOfClass` "/Game/Blueprints/Tile.Tile_C"))
  (for _array_element _outactors
    (`/Game/Blueprints/Tile.Setup` _array_element)))

(fn `UserConstructionScript`)

(fn `Vector Path to Actor`
  (params (Start :type "Actor Object Reference") (Goal :type "Actor Object Reference"))
  (returns (Path :type "Array of Vector Structure"))
  (locals (tPath :type "Array of Vector Structure"))
  (bind _path (`self.Path to Actor` Start Goal))
  (for _array_element _path
    (bind _point (`/Game/Blueprints/Utility/PathFindingLib.Index to Point` _array_element (`self.Width`)))
    (bind _vector (`self.Grid Point to Vector` _point))
    (`KismetArrayLibrary.Array_Add` (`local.tPath`) _vector))
  (return (`local.tPath`)))

(fn `Vector to Grid Point`
  (params (Vector :type "Vector Structure"))
  (returns (Point :type "Vector2D Structure"))
  (bind _returnvalue (`KismetMathLibrary.Conv_IntToDouble` (`self.Offset`)))
  (bind _returnvalue_2 (`KismetMathLibrary.Conv_IntToDouble` (`self.Tile Size`)))
  (return (`KismetMathLibrary.MakeVector2D` (`KismetMathLibrary.Conv_IntToDouble` (`KismetMathLibrary.Round` (/ (- (.x Vector) _returnvalue) _returnvalue_2))) (`KismetMathLibrary.Conv_IntToDouble` (`KismetMathLibrary.Round` (/ (- (.y Vector) _returnvalue) _returnvalue_2))))))