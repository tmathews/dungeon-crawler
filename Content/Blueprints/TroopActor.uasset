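; Troop actor that displays the enemy side of a battle as three EnemySprite child actors labeled A, B and C.
; It binds to MyGameState battle events to show a sprite per troop fighter and hide them when battle ends.
; Target requests make living fighters selectable, confirm or cancel locks them, and a sprite's selection updates Troop.Selected while deselecting the others.
; SetTroop only prints the troop name.
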(event `self.ReceiveBeginPlay`
  ;[1 1 1] Bind Events and initiate each sprite
  (bind _asmy_game_state (cast `/Game/MyGameState` (`GameplayStatics.GetGameState`)))
  (bind _output_get (set `self.Game State` _asmy_game_state))
  (add `/Game/MyGameState.Battle Started` _output_get (delegate `Battle Started Event`))
  (add `/Game/MyGameState.Wants Battle Target` _output_get (delegate `Wants Battle Target Event`))
  (add `/Game/MyGameState.Confirmed Battle Target` _output_get (delegate `Confirmed Battle Target Event`))
  (add `/Game/MyGameState.Cancel Wants Battle Target` _output_get (delegate `Confirmed Battle Target Event`))
  (add `/Game/MyGameState.Battle Ended` _output_get (delegate `Battle Ended Event`))
  (for _array_element (`self.Array of Opponents`)
    (bind _asenemy_sprite (cast `/Game/Blueprints/EnemySprite` _array_element))
    (`/Game/Blueprints/EnemySprite.Set Display` _asenemy_sprite false)
    (add `/Game/Blueprints/EnemySprite.Recieved Selected` _asenemy_sprite (delegate `Recieved Selected`))
    (add `/Game/Blueprints/EnemySprite.Recieved Selected` _asenemy_sprite (delegate `Recieved Selected`))))

(event `Battle Started Event`
  (bind (_name _fighters) (break `/Game/Blueprints/Data/Troop` (`.Troop_70_02866E854E7F934484803B93C7287AC1` (break `/Game/Blueprints/Data/BattleState` (`/Game/MyGameState.Battle State` (`self.Game State`))))))
  ;[1 1 1] Battle Started Initate Troop Sprites
  (for (_array_element _array_index) (`self.Array of Opponents`)
    (bind _asenemy_sprite (cast `/Game/Blueprints/EnemySprite` _array_element))
    (bind _returnvalue (< _array_index (`KismetArrayLibrary.Array_Length` _fighters)))
    (`/Game/Blueprints/EnemySprite.Set Display` _asenemy_sprite _returnvalue)
    (if _returnvalue
      (`/Game/Blueprints/EnemySprite.Set Enemy` _asenemy_sprite (`|GetArrayItem` _fighters _array_index)))))

(event `Confirmed Battle Target Event`
  ;[1 1 1] React to confirmation of target (set all targets to non-selectable)
  (for _array_element (`self.Array of Opponents`)
    (bind _asenemy_sprite (cast `/Game/Blueprints/EnemySprite` _array_element))
    (`/Game/Blueprints/EnemySprite.Set Is Selectable` _asenemy_sprite false)))

(event `Recieved Selected`
  (params (Who :type "/Game/Blueprints/EnemySprite Object Reference"))
  ;[1 1 1] Outside source (like a mouse) set the selected opponent
  (for (_array_element _array_index) (`self.Array of Opponents`)
    (bind _asenemy_sprite (cast `/Game/Blueprints/EnemySprite` _array_element))
    (if (== _asenemy_sprite Who)
      (setmembers `/Game/Blueprints/Data/Troop` :`StructRef` (`.Troop_70_02866E854E7F934484803B93C7287AC1` (break `/Game/Blueprints/Data/BattleState` (`/Game/MyGameState.Battle State` (`self.Game State`)))) :`Selected` _array_index)
      (else
        (`/Game/Blueprints/EnemySprite.Set Is Selected` _asenemy_sprite false false)))))

(event `Battle Ended Event`
  ;[1 1 1] Hide Opponents after battle ends
  (for _array_element (`self.Array of Opponents`)
    (bind _asenemy_sprite (cast `/Game/Blueprints/EnemySprite` _array_element))
    (`/Game/Blueprints/EnemySprite.Set Display` _asenemy_sprite false)))

(event `Wants Battle Target Event`
  (bind (_name _fighters _selected) (break `/Game/Blueprints/Data/Troop` (`.Troop_70_02866E854E7F934484803B93C7287AC1` (break `/Game/Blueprints/Data/BattleState` (`/Game/MyGameState.Battle State` (`self.Game State`))))))
  (bind _returnvalue (`KismetArrayLibrary.Array_Length` _fighters))
  ;[1 1 1] Battle wants a target so set selectables
  (for (_array_element _array_index) (`self.Array of Opponents`)
    (bind _asenemy_sprite (cast `/Game/Blueprints/EnemySprite` _array_element))
    (`/Game/Blueprints/EnemySprite.Set Is Selected` _asenemy_sprite (== _array_index (`KismetMathLibrary.Max` (`KismetMathLibrary.Min` _selected _returnvalue))) false)
    (if (< _array_index _returnvalue)
      (bind _is_alive (`/Game/Blueprints/Utility/BattleLib.Is Fighter Alive` (`|GetArrayItem` _fighters _array_index)))
      (`/Game/Blueprints/EnemySprite.Set Is Selectable` _asenemy_sprite _is_alive)
      (else
        (`/Game/Blueprints/EnemySprite.Set Is Selectable` _asenemy_sprite false)))))

(fn `Set Troop`
  (params (`New Troop` :type "/Game/Blueprints/Data/Troop Structure (by ref)"))
  (`KismetSystemLibrary.PrintString` (`KismetStringLibrary.Concat_StrStr` "Start Troop!" (`.Name_10_82FCE9234DB5A54B46BD7F9204AECAF4` (break `/Game/Blueprints/Data/Troop` `New Troop`)))))

(fn `UserConstructionScript`
  (bind _asenemy_sprite (cast `/Game/Blueprints/EnemySprite` (`ChildActorComponent.ChildActor` (`self.A`))))
  (`TextRenderComponent.K2_SetText` (`/Game/Blueprints/EnemySprite.TextRender` _asenemy_sprite) (`KismetTextLibrary.Conv_StringToText` "A"))
  (bind _asenemy_sprite_2 (cast `/Game/Blueprints/EnemySprite` (`ChildActorComponent.ChildActor` (`self.B`))))
  (`TextRenderComponent.K2_SetText` (`/Game/Blueprints/EnemySprite.TextRender` _asenemy_sprite_2) (`KismetTextLibrary.Conv_StringToText` "B"))
  (bind _asenemy_sprite_3 (cast `/Game/Blueprints/EnemySprite` (`ChildActorComponent.ChildActor` (`self.C`))))
  (`TextRenderComponent.K2_SetText` (`/Game/Blueprints/EnemySprite.TextRender` _asenemy_sprite_3) (`KismetTextLibrary.Conv_StringToText` "C")))