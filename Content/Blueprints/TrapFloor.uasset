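; TrapFloor is a trap floor Blueprint that drops its Plane's collision when an actor overlaps it.
; The overlap calls Open, which disables collision, sets IsOpened and starts a two-second timer by function name.
; The timer runs Close, which restores query and physics collision and prints a debug message.
; Close never resets IsOpened, so the trap opens only once.
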(event `self.ReceiveActorBeginOverlap`
  (params (OtherActor :type "Actor Object Reference"))
  (`self.Open`))

(fn `Close`
  (`PrimitiveComponent.SetCollisionEnabled` (`self.Plane`) "QueryAndPhysics")
  (`KismetSystemLibrary.PrintString` "Closed"))

(fn `Open`
  (if (not (`self.IsOpened`))
    (`PrimitiveComponent.SetCollisionEnabled` (`self.Plane`) "NoCollision")
    (set `self.IsOpened` true)
    (`KismetSystemLibrary.K2_SetTimer` self "Close" 2.0)))

(fn `UserConstructionScript`)