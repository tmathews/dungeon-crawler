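; Enemy battle character that shows the foe as a material billboard with a health bar widget.
; SetFighter stores the fighter's owning battle target and hands it to the EnemyHealthBar widget.
; Shake starts a brief jitter that Tick advances, stepping the billboard at fixed intervals to a random small X or Z offset from its cached origin, then restoring it.
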(event `self.ReceiveBeginPlay`
  (set `self.Origin` (`SceneComponent.RelativeLocation` (`self.MaterialBillboard`))))

(event `self.ReceiveTick`
  (params (DeltaSeconds :type "Float (single-precision)"))
  (`self.Update Shake` DeltaSeconds))

(fn `Set Fighter`
  (params (`New Fighter` :type "/Game/Blueprints/Data/BattleFighter Structure"))
  (bind _output_get (set `self.Battle Target` (`.OwningTarget_60_670E57B4431D1C0AFBBD5AA598A5F17C` (break `/Game/Blueprints/Data/BattleFighter` `New Fighter`))))
  (bind _asenemy_health_bar (cast `/Game/Blueprints/Widgets/EnemyHealthBar` (`WidgetComponent.GetUserWidgetObject` (`self.Widget`))))
  (set `/Game/Blueprints/Widgets/EnemyHealthBar.Battle Target` _output_get _asenemy_health_bar))

(fn `Shake`
  (set `self.Shake Step` 0.0)
  (set `self.Shake Counter` 0)
  (set `self.Shaking` true))

(fn `Update Shake`
  (params (B :type "Float (double-precision)"))
  (bind _returnvalue (select `bool` (`KismetMathLibrary.RandomBool`) :`false` -5.0 :`true` 5.0 :!type "Float (single-precision)"))
  (if (`self.Shaking`)
    (bind _output_get (set `self.Shake Step` (+ (`self.Shake Step`) B)))
    (if (>= (`self.Shake Step`) 0.3)
      (set `self.Shaking` false)
      (`SceneComponent.K2_SetRelativeLocation` (`self.MaterialBillboard`) (`self.Origin`) false false)
      (elif (> (`KismetMathLibrary.FFloor` (/ _output_get 0.05)) (`self.Shake Counter`))
        (`/Engine/EditorBlueprintResources/StandardMacros.IncrementInt` (`self.Shake Counter`)
          (:`  `
            (`SceneComponent.K2_SetRelativeLocation` (`self.MaterialBillboard`) (+ (`self.Origin`) (select `bool` (`KismetMathLibrary.RandomBool`) :`false` (`KismetMathLibrary.MakeVector` _returnvalue) :`true` (`KismetMathLibrary.MakeVector` 0.0 0.0 _returnvalue))) false false)))))))

(fn `UserConstructionScript`)