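; DoorLocked is a door that opens through interaction only when the activating FirstPersonCharacter has the NeededItem.
; ActivateInteraction checks the item and the IsOpen flag, calls Open on success and returns whether it opened the door.
; Open snaps the Door component up to a fixed relative height without animation.
; Close resets it, but nothing in this file calls it.
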(event `self.ReceiveBeginPlay`)

(fn `ActivateInteraction`
  (params (Activator :type "Actor Object Reference"))
  (returns (Success :type Boolean))
  (bind _asfirst_person_character (cast `/Game/FirstPersonBP/Blueprints/FirstPersonCharacter` Activator))
  (bind _has (`/Game/FirstPersonBP/Blueprints/FirstPersonCharacter.HasItem` _asfirst_person_character (`self.NeededItem`)))
  (if (and _has (not (`self.IsOpen`)))
    (`self.Open`)
    (return true)
    (else
      (return false))))

(fn `Close`
  (`SceneComponent.K2_SetRelativeLocation` (`self.Door`) (0.0 0.0 0.0) false false)
  (set `self.IsOpen` false))

(fn `Open`
  (`SceneComponent.K2_SetRelativeLocation` (`self.Door`) (0.0 0.0 175.0) false false)
  (set `self.IsOpen` true))

(fn `UserConstructionScript`)