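; Key is an interactable pickup that gives the player a "Unique Key" inventory item.
; Its Cube component spins continuously around the vertical axis every tick.
; ActivateInteraction casts the activator to FirstPersonCharacter, gives it the non-equipment item, destroys the actor and reports success, or returns false for any other activator.
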(event `self.ReceiveTick`
  (params (DeltaSeconds :type "Float (single-precision)"))
  (`SceneComponent.K2_AddLocalRotation` (`self.Cube`) (`KismetMathLibrary.MakeRotator` 0.0 0.0 (* DeltaSeconds 180.0)) false false))

(fn `ActivateInteraction`
  (params (Activator :type "Actor Object Reference"))
  (returns (Success :type Boolean))
  (bind _asfirst_person_character (cast `/Game/FirstPersonBP/Blueprints/FirstPersonCharacter` Activator)
    (:`then`
      (`/Game/FirstPersonBP/Blueprints/FirstPersonCharacter.GiveItem` _asfirst_person_character (make `/Game/Blueprints/Data/Item` "Unique Key"))
      (`self.K2_DestroyActor`)
      (return true))
    (:`CastFailed`
      (return false))))

(fn `UserConstructionScript`)