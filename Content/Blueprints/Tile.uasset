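; Modular tile actor that builds its floor, ceiling and walls in the construction script and reports which actors occupy it.
; Optional autodetection line-traces six directions for neighbouring Tiles, setting floor and ceiling flags and hashing weighted side hits into a HitMap lookup for the Walls layout.
; Configure then destroys the plane components that layout does not need.
; Box overlap queries report occupying Characters, or class-filtered actors for battle.
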(fn `Autodetect Configuration`
  (locals (Delta :type "Float (double-precision)" :default 400.0) (Hits :type "Array of Integer") (`Hit Sum` :type Integer) (`Hit Count` :type Integer) (`Hit Map` :type "Map of Integer to /Game/Blueprints/Data/TileWallEnum Enum"))
  (bind _hits (`local.Hits`))
  (bind _hit_sum (`local.Hit Sum`))
  (bind _hit_count (`local.Hit Count`))
  (bind _delta (`local.Delta`))
  (bind _delta_2 (`local.Delta`))
  (bind (_value _returnvalue) (`BlueprintMapLibrary.Map_Find` (`local.Hit Map`) (* _hit_sum _hit_count)))
  (bind _hits_2 (`self.Detect Tile` (`KismetMathLibrary.MakeVector` 0.0 0.0 (`local.Delta`))))
  (set `self.Has Ceiling` (not _hits_2))
  (bind _hits_3 (`self.Detect Tile` (`KismetMathLibrary.MakeVector` 0.0 0.0 (* (`local.Delta`) -1.0))))
  (set `self.Has Floor` (not _hits_3))
  (bind _hits_4 (`self.Detect Tile` (`KismetMathLibrary.MakeVector` _delta)))
  (bind _hits_5 (`self.Detect Tile` (`KismetMathLibrary.MakeVector` (* _delta -1.0))))
  (bind _hits_6 (`self.Detect Tile` (`KismetMathLibrary.MakeVector` 0.0 _delta_2)))
  (bind _hits_7 (`self.Detect Tile` (`KismetMathLibrary.MakeVector` 0.0 (* _delta_2 -1.0))))
  (`KismetArrayLibrary.Array_Clear` _hits)
  (bind _returnvalue_2 (`KismetMathLibrary.SelectInt` 9 0 _hits_4))
  (`KismetArrayLibrary.Array_Add` _hits _returnvalue_2)
  (bind _returnvalue_3 (`KismetMathLibrary.SelectInt` 5 0 _hits_5))
  (`KismetArrayLibrary.Array_Add` _hits _returnvalue_3)
  (bind _returnvalue_4 (`KismetMathLibrary.SelectInt` 2 0 _hits_6))
  (`KismetArrayLibrary.Array_Add` _hits _returnvalue_4)
  (bind _returnvalue_5 (`KismetMathLibrary.SelectInt` 7 0 _hits_7))
  (`KismetArrayLibrary.Array_Add` _hits _returnvalue_5)
  (`KismetSystemLibrary.PrintString` (`KismetStringLibrary.Concat_StrStr` (`KismetStringLibrary.Conv_IntToString` _returnvalue_2) ", " (`KismetStringLibrary.Conv_IntToString` _returnvalue_3) "," (`KismetStringLibrary.Conv_IntToString` _returnvalue_4) "," (`KismetStringLibrary.Conv_IntToString` _returnvalue_5)))
  (for _array_element _hits
    (set `local.Hit Sum` (+ _hit_sum _array_element))
    (if (!= _array_element 0)
      (`/Engine/EditorBlueprintResources/StandardMacros.IncrementInt` _hit_count)))
  (if _returnvalue
    (set `self.Walls` _value)
    (else
      (`KismetSystemLibrary.PrintString` "Error finding tile configuration!" false))))

(fn `Configure`
  (locals (`Walls to Discard` :type "Array of StaticMeshComponent Object Reference"))
  (bind _east_wall_plane (`self.East Wall Plane`))
  (bind _walls_to_discard (`local.Walls To Discard`))
  (bind _north_wall_plane (`self.North Wall Plane`))
  (bind _south_wall_plane (`self.South Wall Plane`))
  (bind _west_wall_plane (`self.West Wall Plane`))
  (if (not (`self.Has Floor`))
    (`ActorComponent.K2_DestroyComponent` (`self.Floor Plane`)))
  (if (not (`self.Has Ceiling`))
    (`ActorComponent.K2_DestroyComponent` (`self.Ceiling Plane`)))
  (`KismetArrayLibrary.Array_Clear` _walls_to_discard)
  (`KismetArrayLibrary.Array_Add` _walls_to_discard _north_wall_plane)
  (`KismetArrayLibrary.Array_Add` _walls_to_discard _east_wall_plane)
  (`KismetArrayLibrary.Array_Add` _walls_to_discard _south_wall_plane)
  (`KismetArrayLibrary.Array_Add` _walls_to_discard _west_wall_plane)
  (switch `/Game/Blueprints/Data/TileWallEnum` (`self.Walls`)
    (:`NewEnumerator12`
      (for _array_element _walls_to_discard :!label _label
        (`ActorComponent.K2_DestroyComponent` _array_element)))
    (:`NewEnumerator0`
      _)
    (:`NewEnumerator5`
      (`KismetArrayLibrary.Array_RemoveItem` _walls_to_discard _east_wall_plane)
      (`KismetArrayLibrary.Array_RemoveItem` _walls_to_discard _west_wall_plane)
      (goto _label))
    (:`NewEnumerator6`
      (`KismetArrayLibrary.Array_RemoveItem` _walls_to_discard _north_wall_plane)
      (`KismetArrayLibrary.Array_RemoveItem` _walls_to_discard _south_wall_plane)
      (goto _label))
    (:`NewEnumerator1`
      (`KismetArrayLibrary.Array_RemoveItem` _walls_to_discard _north_wall_plane)
      (goto _label))
    (:`NewEnumerator2`
      (`KismetArrayLibrary.Array_RemoveItem` _walls_to_discard _east_wall_plane)
      (goto _label))
    (:`NewEnumerator3`
      (`KismetArrayLibrary.Array_RemoveItem` _walls_to_discard _south_wall_plane)
      (goto _label))
    (:`NewEnumerator4`
      (`KismetArrayLibrary.Array_RemoveItem` _walls_to_discard _west_wall_plane)
      (goto _label))
    (:`NewEnumerator7`
      (`ActorComponent.K2_DestroyComponent` _south_wall_plane))
    (:`NewEnumerator8`
      (`ActorComponent.K2_DestroyComponent` _west_wall_plane))
    (:`NewEnumerator9`
      (`ActorComponent.K2_DestroyComponent` _north_wall_plane))
    (:`NewEnumerator10`
      (`ActorComponent.K2_DestroyComponent` _east_wall_plane))
    (:`NewEnumerator13`
      (`KismetArrayLibrary.Array_RemoveItem` _walls_to_discard _north_wall_plane)
      (`KismetArrayLibrary.Array_RemoveItem` _walls_to_discard _east_wall_plane)
      (goto _label))
    (:`NewEnumerator14`
      (`KismetArrayLibrary.Array_RemoveItem` _walls_to_discard _north_wall_plane)
      (`KismetArrayLibrary.Array_RemoveItem` _walls_to_discard _west_wall_plane)
      (goto _label))
    (:`NewEnumerator15`
      (`KismetArrayLibrary.Array_RemoveItem` _walls_to_discard _south_wall_plane)
      (`KismetArrayLibrary.Array_RemoveItem` _walls_to_discard _east_wall_plane)
      (goto _label))
    (:`NewEnumerator16`
      (`KismetArrayLibrary.Array_RemoveItem` _walls_to_discard _south_wall_plane)
      (`KismetArrayLibrary.Array_RemoveItem` _walls_to_discard _west_wall_plane)
      (goto _label)))
  (return))

(fn `Detect Tile`
  (params (`Hit Point` :type "Vector Structure"))
  (returns (Hits :type Boolean) (`Tile Hit` :type "/Game/Blueprints/Tile Object Reference"))
  (bind _returnvalue (`self.K2_GetActorLocation`))
  (bind _outhits (`KismetSystemLibrary.LineTraceMultiForObjects` :`Start` _returnvalue :`End` (+ _returnvalue `Hit Point`) :`ObjectTypes` (`|MakeArray` "ObjectTypeQuery1" :!type "EObjectTypeQuery Enum") :`DrawDebugType` "ForOneFrame"))
  (for _array_element _outhits
    (bind _astile (cast `/Game/Blueprints/Tile` (`.HitActor` (`GameplayStatics.BreakHitResult` _array_element))))
    (return true _astile))
  (return false null))

(fn `Is Occupied`
  (returns (Occupied :type Boolean) (Characters :type "Array of Actor Object Reference"))
  (bind _overlappingactors (`PrimitiveComponent.GetOverlappingActors` (`self.Box`) "/Script/Engine.Character"))
  (return (> (`KismetArrayLibrary.Array_Length` _overlappingactors) 0) _overlappingactors))

(fn `Is Occupied for Battle`
  (returns (Occupied :type Boolean) (Characters :type "Array of Actor Object Reference"))
  (locals (Classes :type "Array of Actor Class Reference") (Actors :type "Array of Actor Object Reference"))
  (bind _actors (`local.Actors`))
  (for _array_element (`PrimitiveComponent.GetOverlappingActors` (`self.Box`) "/Script/Engine.Actor")
    (if (`KismetArrayLibrary.Array_Contains` (`local.Classes`) (`GameplayStatics.GetObjectClass` _array_element))
      (`KismetArrayLibrary.Array_Add` (`local.Actors`) _array_element)))
  (return (> (`KismetArrayLibrary.Array_Length` _actors) 0) _actors))

(fn `Setup`
  (if (`self.Autodetect`)
    (`self.Autodetect Configuration`))
  (`self.Configure`)
  (`KismetSystemLibrary.PrintString` (`|GetEnumeratorNameAsString` (`self.Walls`))))

(fn `UserConstructionScript`
  (locals (`Walls To Discard` :type "Array of StaticMeshComponent Object Reference"))
  (`self.Setup`))