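; Elevator lift actor that carries the first-person character between an array of WayPoints actors.
; Player overlap activates it and targets the adjacent index in the GoUp direction, with modulo wrap; exit deactivates it and zeroes step progress.
; Tick lerps relative location between waypoint actor locations at Speed while active or off-target.
; RequestLift sends it to a given waypoint and sets GoUp; GetLiftIndex exposes the current index.
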(event `self.ReceiveActorBeginOverlap`
  (params (OtherActor :type "Actor Object Reference"))
  (bind _currentindex (`self.CurrentIndex`))
  ;[1 1 1] Update Active State and Target Destination upon entry
  (cast `/Game/FirstPersonBP/Blueprints/FirstPersonCharacter` OtherActor)
  (set `self.IsActive` true)
  (set `self.CurrentIndex` _currentindex)
  (bind _output_get (set `self.NextIndex` (mod (+ _currentindex (`KismetMathLibrary.SelectInt` 1 -1 (`self.GoUp`))) (`KismetArrayLibrary.Array_Length` (`self.WayPoints`)))))
  (`KismetSystemLibrary.PrintString` (`KismetStringLibrary.Concat_StrStr` "Hello" (`KismetStringLibrary.Conv_IntToString` _output_get))))

(event `self.ReceiveBeginPlay`
  (`KismetSystemLibrary.Delay` 0.2)
  (set `self.NextIndex` (`self.StartIndex`)))

(event `self.ReceiveActorEndOverlap`
  (params (OtherActor :type "Actor Object Reference"))
  ;[1 1 1] Update Active State and Target Destination upon entry
  (cast `/Game/FirstPersonBP/Blueprints/FirstPersonCharacter` OtherActor)
  (set `self.IsActive` false)
  (set `self.CurrentStep` 0.0)
  (`KismetSystemLibrary.PrintString` "Goodbye"))

(event `self.ReceiveTick`
  (params (DeltaSeconds :type "Float (single-precision)"))
  (bind _waypoints (`self.WayPoints`))
  (bind _currentindex (`self.CurrentIndex`))
  (bind _nextindex (`self.NextIndex`))
  ;[1 1 1] Update Location Based on Active and Target
  (if (or (`self.IsActive`) (!= _currentindex _nextindex))
    (bind _output_get (set `self.CurrentStep` (`KismetMathLibrary.FClamp` (+ (`self.CurrentStep`) (* (`self.Speed`) DeltaSeconds)))))
    (`self.K2_SetActorRelativeLocation` (`KismetMathLibrary.VLerp` (`self.K2_GetActorLocation` (`|GetArrayItem` _waypoints _currentindex)) (`self.K2_GetActorLocation` (`|GetArrayItem` _waypoints _nextindex)) _output_get))
    (if (== _output_get 1.0)
      (set `self.CurrentIndex` _nextindex)
      (set `self.CurrentStep` 0.0))))

(fn `GetLiftIndex`
  (returns (Index :type Integer))
  (return (`self.CurrentIndex`)))

(fn `RequestLift`
  (params (`Return Point` :type "/Game/Blueprints/WayPoint Object Reference") (GoUp :type Boolean))
  (bind _returnvalue (`KismetArrayLibrary.Array_Find` (`self.WayPoints`) `Return Point`))
  (if (> _returnvalue -1)
    (set `self.GoUp` GoUp)
    (bind _output_get (set `self.NextIndex` _returnvalue))
    (`KismetSystemLibrary.PrintString` (`KismetStringLibrary.Concat_StrStr` "requesting next is: " (`KismetStringLibrary.Conv_IntToString` _output_get) " current is: " (`KismetStringLibrary.Conv_IntToString` (`self.CurrentIndex`)) " step is: " (`KismetStringLibrary.Conv_DoubleToString` (`self.CurrentStep`))))))

(fn `UserConstructionScript`)