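; Elevator call button that requests its target lift when activated and displays that lift's current index.
; ActivateInteraction calls RequestLift on TargetLift, passing the button's desired waypoint and up/down direction.
; Tick polls the lift index every frame and writes it to the Status text, showing "G" for index zero.
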(event `self.ReceiveTick`
  (params (DeltaSeconds :type "Float (single-precision)"))
  (bind _index (`/Game/Blueprints/ElevatorLift.GetLiftIndex` (`self.TargetLift`)))
  (`TextRenderComponent.K2_SetText` (`self.Status`) (`KismetTextLibrary.Conv_StringToText` (select `int` _index :`0` "G" :`1` (`KismetStringLibrary.Conv_IntToString` _index)))))

(fn `ActivateInteraction`
  (params (Activator :type "Actor Object Reference"))
  (`/Game/Blueprints/ElevatorLift.RequestLift` (`self.TargetLift`) (`self.DesiredWayPoint`) (`self.GoUp`)))

(fn `UserConstructionScript`)