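; Researcher character Blueprint for an NPC that the player can interact with to hear a short greeting.
; Activating the interaction calls BeginEvent, and the dialog function supplies a single hardcoded line asking whether anything interesting was found.
; It offers no choices, so the choice handler returns false and concluding the event simply reports success.
; The event graph holds only disabled default stubs, and the construction script just calls its parent.
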(fn `ActivateInteraction`
  (params (Activator :type "Actor Object Reference"))
  (returns (Success :type Boolean))
  (`self.Begin Event`)
  (return true))

(fn `Choice Made`
  (params (Index :type Integer))
  (returns (Success :type Boolean))
  (return false))

(fn `Conclude Event`
  (returns (`Is Finished` :type Boolean))
  (return true))

(fn `Get Choices`
  (returns (Choices :type "Array of String") (`Cancel Index` :type Integer))
  (return (`|MakeArray`) -1))

(fn `Get Dialog`
  (returns (Success :type Boolean) (Dialog :type "/Game/Blueprints/Data/Dialog Structure"))
  (return true (make `/Game/Blueprints/Data/Dialog` "Hey! You find anything interesting?")))

(fn `UserConstructionScript`
  (`parent.UserConstructionScript`))