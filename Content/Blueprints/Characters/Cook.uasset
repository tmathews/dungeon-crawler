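; Cook is an interactable character that offers the player a shop through a short dialog.
; Activating it begins an event that supplies a greeting line and Buy or Cancel choices.
; The choice is held in a WantsToBuy flag until the event concludes, when a Buy clears the flag and opens the cook's Store through MyGameState's AccessShop.
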(fn `ActivateInteraction`
  (params (Activator :type "Actor Object Reference"))
  (returns (Success :type Boolean))
  (`self.Begin Event`)
  (return true))

(fn `Choice Made`
  (params (Index :type Integer))
  (returns (Success :type Boolean))
  (set `self.Wants to Buy` (== Index 0))
  (return true))

(fn `Conclude Event`
  (returns (`Is Finished` :type Boolean))
  (if (`self.Wants to Buy`)
    (set `self.Wants to Buy` false)
    (bind _asmy_game_state (cast `/Game/MyGameState` (`GameplayStatics.GetGameState`))
      (:`then`
        (`/Game/MyGameState.Access Shop` _asmy_game_state (`self.Store`)))
      (:`CastFailed`
        _)))
  (return true))

(fn `Get Choices`
  (returns (Choices :type "Array of String") (`Cancel Index` :type Integer))
  (return (`|MakeArray` "Buy" "Cancel") 1))

(fn `Get Dialog`
  (returns (Success :type Boolean) (Dialog :type "/Game/Blueprints/Data/Dialog Structure"))
  (return true (make `/Game/Blueprints/Data/Dialog` "You need some cook'n?")))

(fn `UserConstructionScript`
  (`parent.UserConstructionScript`))