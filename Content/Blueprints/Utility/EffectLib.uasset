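; Battle effect function library that applies skill effects and status ailments to BattleFighter structs.
; ApplyEffect runs health, energy, status, physical and magical passes in turn, each editing the fighter and appending BattleResult dialog entries to a shared array.
; Damage is attack minus defense, boosted on elemental weakness, while status infliction rolls against a chance.
; Separate helpers stamp fighter stats onto skill effects and handle confusion, paralysis, burn, freeze and poison.
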(fn `Apply Burn`
  (params (Fighter :type "/Game/Blueprints/Data/BattleFighter Structure (by ref)") (Results :type "Array of /Game/Blueprints/Data/BattleResult Structure (by ref)"))
  (bind (_name _owningtarget _status _strength _intellect _agility _healthmax) (break `/Game/Blueprints/Data/BattleFighter` Fighter))
  (bind _returnvalue (`KismetMathLibrary.FTrunc` (* _healthmax 0.02)))
  (setmembers `/Game/Blueprints/Data/BattleFighter` :`StructRef` Fighter :`Health Current` _returnvalue)
  (`KismetArrayLibrary.Array_Add` Results (make `/Game/Blueprints/Data/BattleResult` _owningtarget "{owner} took {damage_took} damage from burning." _returnvalue)))

(fn `Apply Confusion`
  (params (Fighter :type "/Game/Blueprints/Data/BattleFighter Structure (by ref)") (Results :type "Array of /Game/Blueprints/Data/BattleResult Structure (by ref)"))
  (bind (_name _owningtarget _status _strength _intellect _agility _healthmax) (break `/Game/Blueprints/Data/BattleFighter` Fighter))
  (bind _returnvalue (`KismetMathLibrary.FTrunc` (* _healthmax 0.05)))
  (setmembers `/Game/Blueprints/Data/BattleFighter` :`StructRef` Fighter :`Health Current` _returnvalue)
  (`KismetArrayLibrary.Array_Add` Results (make `/Game/Blueprints/Data/BattleResult` _owningtarget "{owner} took {damage_took} damage out of confusion." _returnvalue))
  (return))

(fn `Apply Effect`
  (params (Effect :type "/Game/Blueprints/Data/Effect Structure (by ref)") (Fighter :type "/Game/Blueprints/Data/BattleFighter Structure (by ref)"))
  (returns (Results :type "Array of /Game/Blueprints/Data/BattleResult Structure"))
  (locals (Arr :type "Array of /Game/Blueprints/Data/BattleResult Structure"))
  (bind _arr (`local.Arr`))
  (`self.Apply Health Effects` Effect Fighter _arr)
  (`self.Apply Energy Effects` Effect Fighter _arr)
  (`self.Apply Status Effects` Effect Fighter _arr)
  (`self.Apply Physical Effects` Effect Fighter _arr)
  (`self.Apply Magical Effects` Effect Fighter _arr)
  (return _arr))

(fn `Apply Energy Effects`
  (params (Effect :type "/Game/Blueprints/Data/Effect Structure (by ref)") (Fighter :type "/Game/Blueprints/Data/BattleFighter Structure (by ref)") (Results :type "Array of /Game/Blueprints/Data/BattleResult Structure (by ref)"))
  (returns (`Had Effect` :type Boolean))
  (locals (`Energy Changed` :type Integer) (`Energy Restored` :type Integer))
  (bind (_name _owningtarget _status _strength _intellect _agility _healthmax _healthcurrent _energymax _energycurrent) (break `/Game/Blueprints/Data/BattleFighter` Fighter))
  (bind (_name_2 _statusinflict _statusinflictchance _statusfix _healthdeltafixed _healthdeltapercent _energydeltafixed _energydeltapercent) (break `/Game/Blueprints/Data/Effect` Effect))
  (bind _output_get (set `local.Energy Changed` (+ (+ (`local.Energy Changed`) _energydeltafixed) (`KismetMathLibrary.FTrunc` (* (`.EnergyMax_79_E7C9FC6B43AEC6BE0B04D58832993E76` (break `/Game/Blueprints/Data/BattleFighter` Fighter)) _energydeltapercent)))))
  (bind _output_get_2 (set `local.Energy Restored` (`KismetMathLibrary.Min` (- _energymax _energycurrent) _output_get)))
  (if (> _output_get_2 0)
    (setmembers `/Game/Blueprints/Data/BattleFighter` :`StructRef` Fighter :`Energy Current` (+ _energycurrent _output_get_2))
    (`KismetArrayLibrary.Array_Add` Results (select `bool` (>= _output_get_2 0) :`false` (make `/Game/Blueprints/Data/BattleResult` _owningtarget "{owner} lost {energy_lost} energy." 0 _output_get_2) :`true` (make `/Game/Blueprints/Data/BattleResult` _owningtarget "{owner} recovered {energy_recovered} energy." 0 0 0 _output_get_2)))
    (return true)
    (else
      (return false))))

(fn `Apply Frozen`
  (params (Fighter :type "/Game/Blueprints/Data/BattleFighter Structure (by ref)") (Results :type "Array of /Game/Blueprints/Data/BattleResult Structure (by ref)"))
  (`KismetArrayLibrary.Array_Add` Results (make `/Game/Blueprints/Data/BattleResult` (`.OwningTarget_60_670E57B4431D1C0AFBBD5AA598A5F17C` (break `/Game/Blueprints/Data/BattleFighter` Fighter)) "{owner} is frozen and cannot move!"))
  (return))

(fn `Apply Health Effects`
  (params (Effect :type "/Game/Blueprints/Data/Effect Structure (by ref)") (Fighter :type "/Game/Blueprints/Data/BattleFighter Structure (by ref)") (Results :type "Array of /Game/Blueprints/Data/BattleResult Structure (by ref)"))
  (returns (`Had Effect` :type Boolean))
  (locals (`Health Changed` :type Integer) (`Health Restored` :type Integer))
  (bind (_name _owningtarget _status _strength _intellect _agility _healthmax _healthcurrent) (break `/Game/Blueprints/Data/BattleFighter` Fighter))
  (bind (_name_2 _statusinflict _statusinflictchance _statusfix _healthdeltafixed _healthdeltapercent) (break `/Game/Blueprints/Data/Effect` Effect))
  (bind _output_get (set `local.Health Changed` (+ (+ (`local.Health Changed`) _healthdeltafixed) (`KismetMathLibrary.FTrunc` (* (`.HealthMax_48_D9CDACB44B82161A18DE72A3154CC7C8` (break `/Game/Blueprints/Data/BattleFighter` Fighter)) _healthdeltapercent)))))
  (bind _output_get_2 (set `local.Health Restored` (`KismetMathLibrary.Min` (- _healthmax _healthcurrent) _output_get)))
  (if (> _output_get_2 0)
    (setmembers `/Game/Blueprints/Data/BattleFighter` :`StructRef` Fighter :`Health Current` (+ _healthcurrent _output_get_2))
    (`KismetArrayLibrary.Array_Add` Results (select `bool` (>= _output_get_2 0) :`false` (make `/Game/Blueprints/Data/BattleResult` _owningtarget "{owner} took {damage_took} damage." _output_get_2) :`true` (make `/Game/Blueprints/Data/BattleResult` _owningtarget "{owner} recovered {health_recovered} health." 0 0 _output_get_2)))
    (return true)
    (else
      (return false))))

(fn `Apply Magical Effects`
  (params (Effect :type "/Game/Blueprints/Data/Effect Structure (by ref)") (Fighter :type "/Game/Blueprints/Data/BattleFighter Structure (by ref)") (Results :type "Array of /Game/Blueprints/Data/BattleResult Structure (by ref)"))
  (returns (`Had Effect` :type Boolean))
  (bind (_name _statusinflict _statusinflictchance _statusfix _healthdeltafixed _healthdeltapercent _energydeltafixed _energydeltapercent _elementaloverride _stats _statsaffects _statsmodifiers) (break `/Game/Blueprints/Data/Effect` Effect))
  (bind (_name_2 _owningtarget _status _strength _intellect _agility _healthmax _healthcurrent) (break `/Game/Blueprints/Data/BattleFighter` Fighter))
  (bind _returnvalue (* (`.MagicAttack_21_D664CCB7784CB8C354259FA8C30F43A4` (break `/Game/Blueprints/Data/Stats` _stats)) (`.MagicAttack_21_D664CCB7784CB8C354259FA8C30F43A4` (break `/Game/Blueprints/Data/Stats` _statsmodifiers))))
  (if (> _returnvalue 0.0)
    (bind (_stats_2 _element) (`/Game/Blueprints/Utility/BattleLib.Get Stats` Fighter))
    (bind (_strength_2 _weakness) (`/Game/Blueprints/Utility/BattleLib.Get Elemental VS` _element))
    (bind _returnvalue_2 (`KismetMathLibrary.Max` (`KismetMathLibrary.Round` (* (select `bool` (== _weakness _elementaloverride) :`false` 1.0 :`true` 1.5 :!type "Float (single-precision)") (- _returnvalue (`.MagicDefense_22_0C5227352E4E4ADCC9DBD98F154CF94F` (break `/Game/Blueprints/Data/Stats` _stats_2)))))))
    (setmembers `/Game/Blueprints/Data/BattleFighter` :`StructRef` Fighter :`Health Current` (`KismetMathLibrary.Max` (- _healthcurrent _returnvalue_2)))
    (`KismetArrayLibrary.Array_Add` Results (make `/Game/Blueprints/Data/BattleResult` _owningtarget "{owner} took {damage_took} damage!" _returnvalue_2))
    (return true)))

(fn `Apply Paralyzed`
  (params (Fighter :type "/Game/Blueprints/Data/BattleFighter Structure (by ref)") (Results :type "Array of /Game/Blueprints/Data/BattleResult Structure (by ref)"))
  (`KismetArrayLibrary.Array_Add` Results (make `/Game/Blueprints/Data/BattleResult` (`.OwningTarget_60_670E57B4431D1C0AFBBD5AA598A5F17C` (break `/Game/Blueprints/Data/BattleFighter` Fighter)) "{owner} is paralyzed and cannot move!"))
  (return))

(fn `Apply Physical Effects`
  (params (Effect :type "/Game/Blueprints/Data/Effect Structure (by ref)") (Fighter :type "/Game/Blueprints/Data/BattleFighter Structure (by ref)") (Results :type "Array of /Game/Blueprints/Data/BattleResult Structure (by ref)"))
  (returns (`Had Effect` :type Boolean))
  (bind (_name _statusinflict _statusinflictchance _statusfix _healthdeltafixed _healthdeltapercent _energydeltafixed _energydeltapercent _elementaloverride _stats _statsaffects _statsmodifiers) (break `/Game/Blueprints/Data/Effect` Effect))
  (bind (_name_2 _owningtarget _status _strength _intellect _agility _healthmax _healthcurrent) (break `/Game/Blueprints/Data/BattleFighter` Fighter))
  (bind _returnvalue (* (`.Attack_18_5504D10D3F462A915050C6A10C92671C` (break `/Game/Blueprints/Data/Stats` _stats)) (`.Attack_18_5504D10D3F462A915050C6A10C92671C` (break `/Game/Blueprints/Data/Stats` _statsmodifiers))))
  (if (> _returnvalue 0.0)
    (bind (_stats_2 _element) (`/Game/Blueprints/Utility/BattleLib.Get Stats` Fighter))
    (bind (_strength_2 _weakness) (`/Game/Blueprints/Utility/BattleLib.Get Elemental VS` _element))
    (bind _returnvalue_2 (`KismetMathLibrary.Max` (`KismetMathLibrary.Round` (* (select `bool` (== _weakness _elementaloverride) :`false` 1.0 :`true` 1.5 :!type "Float (single-precision)") (- _returnvalue (`.Defense_19_4A48BD2EAE4B1083D30B19A59C6848DC` (break `/Game/Blueprints/Data/Stats` _stats_2)))))))
    (setmembers `/Game/Blueprints/Data/BattleFighter` :`StructRef` Fighter :`Health Current` (`KismetMathLibrary.Max` (- _healthcurrent _returnvalue_2)))
    (`KismetArrayLibrary.Array_Add` Results (make `/Game/Blueprints/Data/BattleResult` _owningtarget "{owner} took {damage_took} damage!" _returnvalue_2))
    (return true)))

(fn `Apply Poison`
  (params (Fighter :type "/Game/Blueprints/Data/BattleFighter Structure (by ref)") (Results :type "Array of /Game/Blueprints/Data/BattleResult Structure (by ref)"))
  (bind (_name _owningtarget _status _strength _intellect _agility _healthmax _healthcurrent) (break `/Game/Blueprints/Data/BattleFighter` Fighter))
  (bind _returnvalue (`KismetMathLibrary.FTrunc` (* _healthmax 0.1)))
  (setmembers `/Game/Blueprints/Data/BattleFighter` :`StructRef` Fighter :`Health Current` (- _healthcurrent _returnvalue))
  (`KismetArrayLibrary.Array_Add` Results (make `/Game/Blueprints/Data/BattleResult` _owningtarget "{owner} took {damage_took} damage from poisoning." _returnvalue))
  (return))

(fn `Apply Status Effects`
  (params (Effect :type "/Game/Blueprints/Data/Effect Structure (by ref)") (Fighter :type "/Game/Blueprints/Data/BattleFighter Structure (by ref)") (Results :type "Array of /Game/Blueprints/Data/BattleResult Structure (by ref)"))
  (returns (`Had Effect` :type Boolean))
  (bind (_name _statusinflict _statusinflictchance) (break `/Game/Blueprints/Data/Effect` Effect))
  (bind (_name_2 _owningtarget _status) (break `/Game/Blueprints/Data/BattleFighter` Fighter))
  (bind (_name_3 _owningtarget_2) (break `/Game/Blueprints/Data/BattleFighter` Fighter))
  (bind (_name_4 _statusinflict_2 _statusinflictchance_2 _statusfix) (break `/Game/Blueprints/Data/Effect` Effect))
  (if (or (and (`|EnumEquality` _statusfix "NewEnumerator0") (`|EnumInequality` _status "NewEnumerator6")) (and (`|EnumInequality` _statusfix "NewEnumerator6") (`|EnumEquality` _statusfix _status)))
    (setmembers `/Game/Blueprints/Data/BattleFighter` :`StructRef` Fighter :`Status` "NewEnumerator6")
    (`KismetArrayLibrary.Array_Add` Results (make `/Game/Blueprints/Data/BattleResult` _owningtarget "{owner} returned to normal condition." 0 0 0 0 false "heal"))
    (return true)
    (elif (`|EnumInequality` _statusinflict "NewEnumerator6")
      (if (<= (`KismetMathLibrary.RandomFloat`) _statusinflictchance)
        (setmembers `/Game/Blueprints/Data/BattleFighter` :`StructRef` Fighter :`Status` _statusinflict)
        (`KismetArrayLibrary.Array_Add` Results (make `/Game/Blueprints/Data/BattleResult` _owningtarget_2 (select `/Game/Blueprints/Data/BattleFighterStatus` _statusinflict :`NewEnumerator1` "{owner} was poisoned!" :`NewEnumerator2` "{owner} became confused!" :`NewEnumerator3` "{owner} is paralysed and may not be able to move!" :`NewEnumerator4` "{owner} became enraged!" :`NewEnumerator7` "{owner} was burned!" :`NewEnumerator8` "{owner} was frozen") 0 0 0 0 false (`|GetEnumeratorNameAsString` _statusinflict)))
        (return true)
        (else
          (`KismetArrayLibrary.Array_Add` Results (make `/Game/Blueprints/Data/BattleResult` _owningtarget_2 "The effect failed."))
          (return false)))
      (else
        (return false)))))

(fn `Get Effect from Fighter Skill`
  (params (Skill :type "/Game/Blueprints/Data/Skill Structure") (Fighter :type "/Game/Blueprints/Data/BattleFighter Structure"))
  (returns (`New Effect` :type "/Game/Blueprints/Data/Effect Structure") (`New Side Effect` :type "/Game/Blueprints/Data/Effect Structure"))
  (bind (_name _description _type _targetchoice _cost _masteringexperience _masteringmax _effect _sideeffect) (break `/Game/Blueprints/Data/Skill` Skill))
  (bind _stats (`/Game/Blueprints/Utility/BattleLib.Get Stats` Fighter))
  (bind _structout (setmembers `/Game/Blueprints/Data/Effect` :`StructRef` _effect :`Stats` _stats))
  (bind _structout_2 (setmembers `/Game/Blueprints/Data/Effect` :`StructRef` _sideeffect :`Stats` _stats))
  (return _structout _structout_2))