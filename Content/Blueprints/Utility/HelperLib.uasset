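; HelperLib is a utility function library for tile-based battle placement and dialog building.
; Four helpers offset an actor's location 400 units along its forward or right axes.
; GetFreePositions feeds the player's four offsets through the first TileManager found, keeping those on existing tiles not occupied for battle.
; StringsToDialog converts an array of strings into Dialog structs.
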(fn `Get Free Positions`
  (returns (Positions :type "Array of Vector Structure"))
  (locals (tPositions :type "Array of Vector Structure") (Valid :type "Array of Vector Structure"))
  (bind _returnvalue (`GameplayStatics.GetPlayerCharacter` null))
  (bind _tpositions (`local.tPositions`))
  (bind _vec (`self.Get Position Front` _returnvalue))
  (`KismetArrayLibrary.Array_Add` _tpositions _vec)
  (bind _vec_2 (`self.Get Position Right` _returnvalue))
  (`KismetArrayLibrary.Array_Add` _tpositions _vec_2)
  (bind _vec_3 (`self.Get Position Left` _returnvalue))
  (`KismetArrayLibrary.Array_Add` _tpositions _vec_3)
  (bind _vec_4 (`self.Get Position Back` _returnvalue))
  (`KismetArrayLibrary.Array_Add` _tpositions _vec_4)
  (bind _manager (`self.Get Tile Manager` null))
  (for _array_element _tpositions
    (bind (_found _tile) (`/Game/Blueprints/TileManager.Get Tile at Vector` _manager _array_element))
    (if _found
      (bind _occupied (`/Game/Blueprints/Tile.Is Occupied for Battle` _tile))
      (if (not _occupied)
        (`KismetArrayLibrary.Array_Add` (`local.Valid`) _array_element))))
  (return (`local.Valid`)))

(fn `Get Position Back`
  (params (Actor :type "Actor Object Reference"))
  (returns (Vec :type "Vector Structure"))
  (return (+ (`Actor.K2_GetActorLocation` Actor) (* (`Actor.GetActorForwardVector` Actor) -400.0))))

(fn `Get Position Front`
  (params (Actor :type "Actor Object Reference"))
  (returns (Vec :type "Vector Structure"))
  (return (+ (`Actor.K2_GetActorLocation` Actor) (* (`Actor.GetActorForwardVector` Actor) 400.0))))

(fn `Get Position Left`
  (params (Actor :type "Actor Object Reference"))
  (returns (Vec :type "Vector Structure"))
  (return (+ (`Actor.K2_GetActorLocation` Actor) (* (`Actor.GetActorRightVector` Actor) -400.0))))

(fn `Get Position Right`
  (params (Actor :type "Actor Object Reference"))
  (returns (Vec :type "Vector Structure"))
  (return (+ (`Actor.K2_GetActorLocation` Actor) (* (`Actor.GetActorRightVector` Actor) 400.0))))

(fn `Get Tile Manager`
  (returns (Manager :type "/Game/Blueprints/TileManager Object Reference"))
  (bind _outactors (`GameplayStatics.GetAllActorsOfClass` null "/Game/Blueprints/TileManager.TileManager_C"))
  (for _array_element _outactors
    (return _array_element)))

(fn `Strings to Dialog`
  (params (Strings :type "Array of String"))
  (returns (Dialogs :type "Array of /Game/Blueprints/Data/Dialog Structure"))
  (locals (tArr :type "Array of /Game/Blueprints/Data/Dialog Structure"))
  (for _array_element Strings
    (`KismetArrayLibrary.Array_Add` (`local.tArr`) (make `/Game/Blueprints/Data/Dialog` _array_element)))
  (return (`local.tArr`)))