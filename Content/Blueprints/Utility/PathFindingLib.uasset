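; Pathfinding utility that finds a route between two cell indices on a flattened 2D boolean grid.
; Find Path runs an unweighted breadth-first search, using Get Neighbors to gather in-bounds true cells along Directions offsets and recording each in a CameFrom map.
; Get Path walks that map back from the goal, returning indices in goal-to-start order, or just the goal when it is unreached.
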(fn `Find Path`
  (params (Grid :type "Array of Boolean") (Width :type Integer) (Start :type Integer) (Goal :type Integer))
  (returns (Path :type "Array of Integer"))
  (locals (Frontier :type "Array of Integer") (`Came From` :type "Map of Integer to Object Object Reference") (Current :type Integer))
  (bind _returnvalue (`KismetArrayLibrary.Array_Length` Grid))
  (bind _frontier (`local.Frontier`))
  (bind _frontier_2 (`local.Frontier`))
  (if (!= Start Goal)
    (if (and (< Start _returnvalue) (< Goal _returnvalue))
      (`BlueprintMapLibrary.Map_Add` (`local.Came From`) Start -1)
      (`KismetArrayLibrary.Array_Add` _frontier Start)
      (while (and (!= (`KismetArrayLibrary.Array_Length` _frontier) 0) (!= (`local.Current`) Goal))
        (bind _output_get (set `local.Current` (`|GetArrayItem` _frontier_2 0)))
        (`KismetArrayLibrary.Array_Remove` _frontier_2 0)
        (if (!= _output_get Goal)
          (bind _neighbors (`self.Get Neighbors` Grid Width (`KismetMathLibrary.FCeil` (/ (`KismetMathLibrary.Conv_IntToDouble` _returnvalue) (`KismetMathLibrary.Conv_IntToDouble` Width))) _output_get))
          (for _array_element _neighbors
            (if (not (`BlueprintMapLibrary.Map_Contains` (`local.Came From`) _array_element))
              (`BlueprintMapLibrary.Map_Add` (`local.Came From`) _array_element _output_get)
              (`KismetArrayLibrary.Array_Add` (`local.Frontier`) _array_element)))))
      (bind _path (`self.Get Path` Start Goal (`local.Came From`)))
      (return _path)
      (else
        _)))
  (return))

(fn `Get Neighbors`
  (params (Grid :type "Array of Boolean (by ref)") (Width :type Integer) (Height :type Integer) (Index :type Integer))
  (returns (Neighbors :type "Array of Integer"))
  (locals (Directions :type "Array of Vector2D Structure") (tNeighbors :type "Array of Integer"))
  (bind _point (`self.Index to Point` Index Width))
  (for _array_element (`local.Directions`)
    (bind _returnvalue (+ _point _array_element))
    (bind _index (`self.Point to Index` Width _returnvalue))
    (bind (_x _y) (`KismetMathLibrary.BreakVector2D` _returnvalue))
    (bind _returnvalue_2 (`KismetMathLibrary.FFloor` _x))
    (bind _returnvalue_3 (`KismetMathLibrary.FFloor` _y))
    (if (and (< _returnvalue_2 Width) (>= _returnvalue_2 0) (< _returnvalue_3 Height) (>= _returnvalue_3 0))
      (if (`|GetArrayItem` Grid _index)
        (`KismetArrayLibrary.Array_Add` (`local.tNeighbors`) _index))))
  (return (`local.tNeighbors`)))

(fn `Get Path`
  (params (Start :type Integer) (Goal :type Integer) (`Came From` :type "Map of Integer to Integer (by ref)"))
  (returns (Path :type "Array of Integer"))
  (locals (Current :type Integer) (tPath :type "Array of Integer"))
  (bind (_value _returnvalue) (`BlueprintMapLibrary.Map_Find` `Came From` (`local.Current`)))
  (bind _output_get (set `local.Current` Goal))
  (set `local.tPath` (`|MakeArray` _output_get))
  (while (!= Start (`local.Current`))
    (if _returnvalue
      (bind _output_get_2 (set `local.Current` _value))
      (`KismetArrayLibrary.Array_Add` (`local.tPath`) _output_get_2)
      (else
        (set `local.Current` Start))))
  (return (`local.tPath`)))

(fn `Index to Point`
  (params (Index :type Integer) (Width :type Integer))
  (returns (Point :type "Vector2D Structure"))
  (bind _returnvalue (/ Index Width))
  (return (`KismetMathLibrary.MakeVector2D` (`KismetMathLibrary.Conv_IntToDouble` (- Index (* _returnvalue Width))) (`KismetMathLibrary.Conv_IntToDouble` _returnvalue))))

(fn `Point Inside Grid`
  (params (Point :type "Vector2D Structure") (Width :type Integer) (Height :type Integer))
  (returns (`Is Inside` :type Boolean))
  (bind (_x _y) (`KismetMathLibrary.BreakVector2D` Point))
  (return (and (< (`KismetMathLibrary.FFloor` _x) Width) (< (`KismetMathLibrary.FFloor` _y) Height))))

(fn `Point to Index`
  (params (Width :type Integer) (Point :type "Vector2D Structure"))
  (returns (Index :type Integer))
  (bind (_x _y) (`KismetMathLibrary.BreakVector2D` Point))
  (return (+ (`KismetMathLibrary.FFloor` _x) (`KismetMathLibrary.FFloor` (* Width _y)))))