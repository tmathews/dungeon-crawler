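; AnimationLib is a utility Blueprint whose ShakeTargetOfResult function gives visual hit feedback for a battle result with nonzero damage.
; If the result's owning target is the first enum entry, apparently the player, it plays a DamagedShake world camera shake at the player character's location.
; For any other target, it searches all EnemyBattleCharacter actors and calls Shake on those with a matching BattleTarget.
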(fn `Shake Target of Result`
  (params (Result :type "/Game/Blueprints/Data/BattleResult Structure"))
  (bind (_owningtarget _dialog _damagetook) (break `/Game/Blueprints/Data/BattleResult` Result))
  (if (!= _damagetook 0)
    (if (`|EnumInequality` _owningtarget "NewEnumerator0")
      (bind _outactors (`GameplayStatics.GetAllActorsOfClass` null "/Game/Blueprints/EnemyBattleCharacter.EnemyBattleCharacter_C"))
      (for _array_element _outactors
        (if (== (`/Game/Blueprints/EnemyBattleCharacter.Battle Target` _array_element) _owningtarget)
          (`/Game/Blueprints/EnemyBattleCharacter.Shake` _array_element)))
      (else
        (`GameplayStatics.PlayWorldCameraShake` null "/Game/Blueprints/DamagedShake.DamagedShake_C" (`Actor.K2_GetActorLocation` (`GameplayStatics.GetPlayerCharacter` null)) 0.0 400.0)))))