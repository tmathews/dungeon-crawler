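; Blueprint function library for inventory and crafting, handling items and world materials.
; Give, take and has-check functions match entries by name, stacking counts or clamping removals at zero, with helpers formatting acquisition strings.
; Crafting functions check and consume required materials on the GameState's Player, then grant output by inventory type.
; Equipment output is a hardcoded "Useless Hat", and the give functions print debug text.
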(fn `Give Items`
  (params (Array :type "Array of /Game/Blueprints/Data/Item Structure (by ref)") (`Items to Recieve` :type "Array of /Game/Blueprints/Data/Item Structure"))
  (locals (Found :type Boolean))
  (`KismetSystemLibrary.PrintString` null (`KismetStringLibrary.Concat_StrStr` "time to giv " (`KismetStringLibrary.Conv_IntToString` (`KismetArrayLibrary.Array_Length` `Items to Recieve`))))
  (for _array_element `Items to Recieve`
    (set `local.Found` false)
    (bind (_name _description _targetchoice _canuseinbattle _count) (break `/Game/Blueprints/Data/Item` _array_element))
    (`KismetSystemLibrary.PrintString` null _name)
    (for (_ _array_index) Array
      (bind _output (`|GetArrayItem` Array _array_index))
      (bind (_name_2 _description_2 _targetchoice_2 _canuseinbattle_2 _count_2) (break `/Game/Blueprints/Data/Item` _output))
      (if (`KismetStringLibrary.EqualEqual_StrStr` _name_2 _name)
        (`KismetSystemLibrary.PrintString` null (`KismetStringLibrary.Concat_StrStr` "Counts" (`KismetStringLibrary.Conv_IntToString` _count_2) " " (`KismetStringLibrary.Conv_IntToString` _count)))
        (setmembers `/Game/Blueprints/Data/Item` :`StructRef` _output :`Count` (+ _count_2 _count))
        (set `local.Found` true)))
    (if (not (`local.Found`))
      (`KismetArrayLibrary.Array_Add` Array _array_element))))

(fn `Give Materials`
  (params (Array :type "Array of /Game/Blueprints/Data/WorldMaterial Structure (by ref)") (`Materials to Recieve` :type "Array of /Game/Blueprints/Data/WorldMaterial Structure"))
  (locals (Found :type Boolean))
  (`KismetSystemLibrary.PrintString` null (`KismetStringLibrary.Concat_StrStr` "mats count " (`KismetStringLibrary.Conv_IntToString` (`KismetArrayLibrary.Array_Length` `Materials to Recieve`))))
  (for _array_element `Materials to Recieve`
    (bind (_name _description _count) (break `/Game/Blueprints/Data/WorldMaterial` _array_element))
    (`KismetSystemLibrary.PrintString` null (`KismetStringLibrary.Concat_StrStr` _name))
    (set `local.Found` false)
    (for (_ _array_index) Array
      (bind _output (`|GetArrayItem` Array _array_index))
      (bind (_name_2 _description_2 _count_2) (break `/Game/Blueprints/Data/WorldMaterial` _output))
      (if (`KismetStringLibrary.EqualEqual_StrStr` _name_2 _name)
        (setmembers `/Game/Blueprints/Data/WorldMaterial` :`StructRef` _output :`Count` (+ _count_2 _count))
        (set `local.Found` true)))
    (if (not (`local.Found`))
      (`KismetArrayLibrary.Array_Add` Array _array_element))))

(fn `Has Materials`
  (params (Array :type "Array of /Game/Blueprints/Data/WorldMaterial Structure") (`Materials Needed` :type "Array of /Game/Blueprints/Data/WorldMaterial Structure"))
  (returns (`Has Materials Needed` :type Boolean))
  (locals (`Has Current` :type Boolean) (`Found Current` :type Boolean))
  (for _array_element `Materials Needed`
    (set `local.Has Current` false)
    (set `local.Found Current` false)
    (for (_ _array_index) Array
      (bind (_name _description _count) (break `/Game/Blueprints/Data/WorldMaterial` (`|GetArrayItem` Array _array_index)))
      (bind (_name_2 _description_2 _count_2) (break `/Game/Blueprints/Data/WorldMaterial` _array_element))
      (if (`KismetStringLibrary.EqualEqual_StrStr` _name _name_2)
        (set `local.Found Current` true)
        (set `local.Has Current` (>= _count _count_2))))
    (if (not (and (`local.Found Current`) (`local.Has Current`)))
      (return false)))
  (return true))

(fn `Item to Aquired String`
  (params (Item :type "/Game/Blueprints/Data/Item Structure"))
  (returns (ReturnValue :type String))
  (bind (_name _description _targetchoice _canuseinbattle _count) (break `/Game/Blueprints/Data/Item` Item))
  (return (`KismetStringLibrary.Concat_StrStr` (`KismetStringLibrary.Conv_IntToString` _count) "x " "\"" _name "\"")))

(fn `Material to Aquired String`
  (params (Material :type "/Game/Blueprints/Data/WorldMaterial Structure"))
  (returns (ReturnValue :type String))
  (bind (_name _description _count) (break `/Game/Blueprints/Data/WorldMaterial` Material))
  (return (`KismetStringLibrary.Concat_StrStr` (`KismetStringLibrary.Conv_IntToString` _count) "x " "\"" _name "\"")))

(fn `Player Can Make Craftable`
  (params (Craftable :type "/Game/Blueprints/Data/Craftable Structure"))
  (returns (`Can Craft` :type Boolean))
  (bind _asmy_game_state (cast `/Game/MyGameState` (`GameplayStatics.GetGameState` null)))
  (bind _has_materials_needed (`self.Has Materials` (`.Materials_95_4062056B445BDA02FD4D388FADED9EEB` (break `/Game/Blueprints/Data/BattleFighter` (`/Game/MyGameState.Player` _asmy_game_state))) (`.RequiredMaterials_35_722959094A329D65C127A2B038986779` (break `/Game/Blueprints/Data/Craftable` Craftable))))
  (return _has_materials_needed))

(fn `Player Make Craftable`
  (params (Craftable :type "/Game/Blueprints/Data/Craftable Structure (by ref)"))
  (bind (_name _inventorytype _requiredmaterials) (break `/Game/Blueprints/Data/Craftable` Craftable))
  (bind _asmy_game_state (cast `/Game/MyGameState` (`GameplayStatics.GetGameState` null)))
  (bind (_name_2 _owningtarget _status _strength _intellect _agility _healthmax _healthcurrent _energymax _energycurrent _equipment _items _materials) (break `/Game/Blueprints/Data/BattleFighter` (`/Game/MyGameState.Player` _asmy_game_state)))
  (`self.Take Materials` _materials _requiredmaterials)
  (switch `/Game/Blueprints/Data/InventoryType` _inventorytype
    (:`NewEnumerator0`
      (`self.Give Items` _items (`|MakeArray` (make `/Game/Blueprints/Data/Item` _name "" "NewEnumerator0" false 1))))
    (:`NewEnumerator1`
      (`KismetArrayLibrary.Array_Add` _equipment (make `/Game/Blueprints/Data/Equipment` "Useless Hat" false "NewEnumerator0" "NewEnumerator4" (make `/Game/Blueprints/Data/Stats` 0.0))))
    (:`NewEnumerator2`
      (`self.Give Materials` _materials (`|MakeArray` (make `/Game/Blueprints/Data/WorldMaterial` _name "" 1))))))

(fn `Take Materials`
  (params (Array :type "Array of /Game/Blueprints/Data/WorldMaterial Structure") (`Materials to Take` :type "Array of /Game/Blueprints/Data/WorldMaterial Structure"))
  (for _array_element `Materials to Take`
    (for (_ _array_index) Array
      (bind _output (`|GetArrayItem` Array _array_index))
      (bind (_name _description _count) (break `/Game/Blueprints/Data/WorldMaterial` _output))
      (bind (_name_2 _description_2 _count_2) (break `/Game/Blueprints/Data/WorldMaterial` _array_element))
      (if (`KismetStringLibrary.EqualEqual_StrStr` _name _name_2)
        (setmembers `/Game/Blueprints/Data/WorldMaterial` :`StructRef` _output :`Count` (`KismetMathLibrary.Max` (- _count _count_2)))))))