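; LanguageLib is a utility function library that turns battle results into readable dialog text.
; Translate Battle Result looks up the owning fighter in the battle state's fighter array, then passes it to Translate Fighter Result.
; That function fills placeholder tokens in the result's dialog template through chained string replacements, inserting the fighter's name, damage, health and energy changes, and item and skill names.
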(fn `Translate Battle Result`
  (params (Result :type "/Game/Blueprints/Data/BattleResult Structure (by ref)") (`Battle State` :type "/Game/Blueprints/Data/BattleState Structure (by ref)"))
  (returns (`New String` :type String))
  (bind _fighter (`/Game/Blueprints/Utility/BattleLib.Get Fighter from Array` (`.Fighters_26_3691F9CB490EC90F9F29FC910D49F439` (break `/Game/Blueprints/Data/BattleState` `Battle State`)) (`.OwningTarget_16_1B4140FF4A5582A43D6F13B03024593E` (break `/Game/Blueprints/Data/BattleResult` Result))))
  (bind _returnvalue (`self.Translate Fighter Result` Result _fighter))
  (return _returnvalue))

(fn `Translate Fighter Result`
  (params (BattleResult :type "/Game/Blueprints/Data/BattleResult Structure (by ref)") (Fighter :type "/Game/Blueprints/Data/BattleFighter Structure (by ref)"))
  (returns (ReturnValue :type String))
  (bind (_owningtarget _dialog _damagetook _energylost _healthrecovered _energyrecovered _diddie _effectanimation _itemname _skillname) (break `/Game/Blueprints/Data/BattleResult` BattleResult))
  (return (`KismetStringLibrary.Replace` (`KismetStringLibrary.Replace` (`KismetStringLibrary.Replace` (`KismetStringLibrary.Replace` (`KismetStringLibrary.Replace` (`KismetStringLibrary.Replace` (`KismetStringLibrary.Replace` _dialog "{owner}" (`.Name_2_A97317114846E9113D0ACB8D295A3CA6` (break `/Game/Blueprints/Data/BattleFighter` Fighter))) "{damage_took}" (`KismetStringLibrary.Conv_IntToString` _damagetook)) "{health_recovered}" (`KismetStringLibrary.Conv_IntToString` _healthrecovered)) "{energy_lost}" (`KismetStringLibrary.Conv_IntToString` _energylost)) "{energy_recovered}" (`KismetStringLibrary.Conv_IntToString` _energyrecovered)) "{item_name}" _itemname) "{skill_name}" _skillname)))