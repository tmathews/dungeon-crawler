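; EnemySprite is an enemy actor for battles that the player selects as a target with the mouse.
; While selectable and in battle, Tick line-traces from the cursor, selects the hovered enemy and broadcasts RecievedSelected.
; The Okay input confirms a selected, hovered enemy through MyGameState.
; Setter functions toggle battle display, selectability and the selection arrow, while SetEnemy is an empty stub.
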(event `self.ReceiveBeginPlay`
  ;[1 1 1] Required for input!
  (`self.EnableInput` (`GameplayStatics.GetPlayerController` 0)))

(event `self.ReceiveTick`
  (params (DeltaSeconds :type "Float (single-precision)"))
  ;[1 1 1] Check mouse hovering selection
  (if (and (`self.Is Selectable`) (`self.Is in Battle`))
    (bind (_enemy _success) (`self.Get Mouse Over Target`))
    (if (and (== _enemy self) _success (not (`self.Is Selected`)))
      (`self.Set Is Selected` true true))))

(event `InputAction|Okay` :consume false
  (params (Key :type "Key Structure"))
  ;[1 1 1] Confirm target selection by InputAction Okay (TODO refactor out mouse check!)
  (:`Pressed`
    (if (and (and (`self.Is Selectable`) (`self.Is in Battle`)) (`self.Is Selected`))
      (bind (_enemy _success) (`self.Get Mouse Over Target`))
      (if (and _success (== _enemy self))
        (bind _asmy_game_state (cast `/Game/MyGameState` (`GameplayStatics.GetGameState`)))
        (`/Game/MyGameState.Confirmed Battle Target` _asmy_game_state)))))

(fn `Get Mouse Over Target`
  (returns (Enemy :type "/Game/Blueprints/EnemySprite Object Reference") (Success :type Boolean))
  (bind (_worldlocation _worlddirection) (`PlayerController.DeprojectMousePositionToWorld` (`GameplayStatics.GetPlayerController` 0)))
  (bind _outhits (`KismetSystemLibrary.LineTraceMultiForObjects` :`Start` _worldlocation :`End` (+ _worldlocation (* _worlddirection 1000.0)) :`ObjectTypes` (`|MakeArray` "ObjectTypeQuery1" "ObjectTypeQuery2" "ObjectTypeQuery3" :!type "EObjectTypeQuery Enum") :`bIgnoreSelf` false))
  (for _array_element _outhits
    (bind _asenemy_sprite (cast `/Game/Blueprints/EnemySprite` (`.HitActor` (`GameplayStatics.BreakHitResult` _array_element))))
    (return _asenemy_sprite true))
  (return null false))

(fn `Print State`
  (`KismetSystemLibrary.PrintString` (`KismetStringLibrary.Concat_StrStr` (`KismetTextLibrary.Conv_TextToString` (`TextRenderComponent.Text` (`self.TextRender`))) " >> " (`KismetStringLibrary.Concat_StrStr` "is selectable " (`KismetStringLibrary.Conv_BoolToString` (`self.Is Selected`)) " is in battle " (`KismetStringLibrary.Conv_BoolToString` (`self.Is in Battle`)) " is selected " (`KismetStringLibrary.Conv_BoolToString` (`self.Is Selectable`))))))

(fn `Set Display`
  (params (Visible :type Boolean))
  (`SceneComponent.SetVisibility` (`self.Scene`) Visible true)
  (set `self.Is in Battle` Visible)
  (`SceneComponent.SetVisibility` (`self.Selection Arrow`) false false))

(fn `Set Enemy`
  (params (`New Enemy` :type "/Game/Blueprints/Data/BattleFighter Structure (by ref)")))

(fn `Set Is Selectable`
  (params (Selectable :type Boolean))
  (bind _output_get (set `self.Is Selectable` Selectable))
  (`SceneComponent.SetVisibility` (`self.Selection Arrow`) _output_get false))

(fn `Set Is Selected`
  (params (`Is Selected` :type Boolean) (Propagate :type Boolean :default false))
  (bind _output_get (set `self.Is Selected` `Is Selected`))
  (`SceneComponent.SetVisibility` (`self.Selection Arrow`) _output_get false)
  (if Propagate
    (`self.Recieved Selected` self)))

(fn `UserConstructionScript`)