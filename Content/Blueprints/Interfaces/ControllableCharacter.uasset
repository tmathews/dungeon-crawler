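; ControllableCharacter is an interface in the Interfaces folder for characters that supply their own AI behavior settings.
; Its getters expose patrol points, a desired AI type enum, wander mode and range, decision wait time, and chase target with a chasing flag.
; InitiateContact takes an Actor and returns a boolean.
; The graphs hold only empty or default returns, leaving the behavior to implementers.
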(fn `Get Chase Target`
  (returns (Chasing :type Boolean) (`Chase Target` :type "Actor Object Reference"))
  (return false null))

(fn `Get Decision Wait Time`
  (returns (Time :type "Float (double-precision)"))
  (return 0.0))

(fn `Get Desired AI Type`
  (returns (Type :type "/Game/Blueprints/Data/AIMovementType Enum"))
  (return "NewEnumerator0"))

(fn `Get Patrol Points`
  (returns (`Patrol Points` :type "Array of /Game/Blueprints/WayPoint Object Reference"))
  (return))

(fn `Get True Wander`
  (returns (`True Wander` :type Boolean))
  (return false))

(fn `Get Wander Range`
  (returns (Range :type Integer))
  (return 0))

(fn `Initiate Contact`
  (params (Actor :type "Actor Object Reference"))
  (returns (Success :type Boolean))
  (return false))